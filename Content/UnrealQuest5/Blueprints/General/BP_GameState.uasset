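; Game state Blueprint that runs the session: game timer, score and level progression, game over and pause menu toggling.
; The player's start dispatcher begins a one-second timer, 2D sound and game-only input, while health component death broadcasts game over.
; Points are checked against DT_LevelProgression thresholds to raise the level, with time, points and level broadcast through dispatchers.
; It also disables Nanite by console command and keeps PlaySound from overlapping sounds.
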(event `self.ReceiveBeginPlay`
  (bind _returnvalue (`GameplayStatics.GetPlayerCharacter` 0))
  (bind _returnvalue_2 (`GameplayStatics.GetPlayerCharacter` 0))
  (bind _returnvalue_3 (`self.GetComponentByClass` _returnvalue_2 "/Game/UnrealQuest5/Blueprints/Components/BPC_HealthComponent.BPC_HealthComponent_C"))
  (`|ExecutionSequence`
    (:`then_0`
      (`/Engine/EditorBlueprintResources/StandardMacros.IsValid` _returnvalue
        (:`Is Valid`
          (bind _asbp_player_zdcharacter (cast `/Game/UnrealQuest5/Blueprints/Characters/BP_PlayerZDCharacter` _returnvalue))
          (set `self.Player Character Ref` _asbp_player_zdcharacter)
          (add `/Game/UnrealQuest5/Blueprints/Characters/BP_PlayerZDCharacter.StartGameDispatcher` (`self.Player Character Ref`) (delegate `StartGameDispatcher_Event`)))))
    (:`then_1`
      (`/Engine/EditorBlueprintResources/StandardMacros.IsValid` _returnvalue_2
        (:`Is Valid`
          (`/Engine/EditorBlueprintResources/StandardMacros.IsValid` _returnvalue_3
            (:`Is Valid`
              (add `/Game/UnrealQuest5/Blueprints/Components/BPC_HealthComponent.OnDeath` _returnvalue_3 (delegate `OnDeath_Event`)))))))
    (:`then_2`
      (`KismetSystemLibrary.ExecuteConsoleCommand` "r.Nanite 0" null)
      (`KismetSystemLibrary.ExecuteConsoleCommand` "DisableAllscreenMessages" null)
      (bind _asbp_game_instance (cast `/Game/UnrealQuest5/Blueprints/General/BP_GameInstance` (`GameplayStatics.GetGameInstance`)))
      (set `self.GameInstance` _asbp_game_instance))
    (:`then_3`
      (bind _asbp_hud (cast `/Game/_HentaiShooter/HUD/BP_HUD` (`PlayerController.GetHUD` (`GameplayStatics.GetPlayerController` 0))))
      (set `self.BP HUD` _asbp_hud))))

(event `OnDeath_Event`
  (`self.OnGameOver`))

(event `StartGameDispatcher_Event`
  ;[1 1 1] Game Start
  (`self.UpdatePoints` 0)
  (bind _returnvalue (`KismetSystemLibrary.K2_SetTimerDelegate` (delegate `UpdateTime`) 1.0 true))
  (set `self.GameTimerHandle` _returnvalue)
  (`GameplayStatics.SpawnSound2D` null 1.0 1.0 0.0 null false false)
  (`WidgetBlueprintLibrary.SetInputMode_GameOnly` (`GameplayStatics.GetPlayerController` 0) true))

(event `UpdateTime`
  ;[1 1 1] Game Start
  ;;[1 1 1] StartUpdateTime
  (bind _result (`/Engine/EditorBlueprintResources/StandardMacros.IncrementInt` (`self.TimeSinceGameStart`))
    (:`  `
      (`self.UpdateTimeDispatcher` _result))))

(event `UpdatePoints`
  (params (Points :type Integer))
  ;[1 1 1] Update Score and Level
  (bind _output_get (set `self.CurrentPoints` (+ (`self.CurrentPoints`) Points)))
  (bind _returnvalue (`|GetDataTableRow` "/Game/_HentaiShooter/Core/DT_LevelProgression.DT_LevelProgression" "Levels")
    (:`then`
      (bind _output (`|GetArrayItem` (`.Points_7_A2CCE91044C8B29DA8E2D7BE8D593A97` (break `/Game/_HentaiShooter/Core/LevelProgression` _returnvalue)) (`self.CurrentLevel`)))
      (`self.UpdatePointsDispatcher` _output_get _output)
      (if (>= (`self.CurrentPoints`) _output)
        (bind _result (`/Engine/EditorBlueprintResources/StandardMacros.IncrementInt` (`self.CurrentLevel`))
          (:`  `
            (`self.UpdateLevelDispatcher` _result :!label _label)))))
    (:`RowNotFound`
      (goto _label))))

(event `PlaySound`
  (params (Cue :type "SoundCue Object Reference") (Location :type "Vector Structure"))
  (bind _sound (`self.Sound`))
  ;[1 1 1] PlaySound
  (`/Engine/EditorBlueprintResources/StandardMacros.IsValid` _sound
    (:`Is Valid`
      (if (not (`AudioComponent.IsPlaying` _sound))
        (bind _returnvalue (`GameplayStatics.SpawnSoundAtLocation` Cue Location (struct) 1.0 1.0 0.0 null null :!label _label_2))
        (set `self.Sound` _returnvalue)))
    (:`Is Not Valid`
      (goto _label_2))))

(event `PauseGame`
  (bind _bp_hud (`self.BP HUD`))
  ;[1 1 1] PauseGame
  (if (`GameplayStatics.IsGamePaused`)
    (`/Game/_HentaiShooter/HUD/BP_HUD.Close Menu` _bp_hud)
    (else
      (`/Game/_HentaiShooter/HUD/BP_HUD.Open Menu` _bp_hud))))

(fn `UserConstructionScript`)