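; Base-style PaperZD enemy character that faces its movement or target, attacks with a child-actor sword and drops loot on death.
; Tick derives an eight-way animation direction from velocity, or from the target when idle; attacks lock it toward the target.
; The sword hitbox toggles on directional sockets, and damage flickers sprite material opacity.
; Health component death unpossesses, disables collision and spawns loot; off-screen timed destruction is present but disconnected.
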(event `self.ReceiveTick`
  (params (DeltaSeconds :type "Float (single-precision)"))
  (bind (_returnvalue_x _returnvalue_y) (`KismetMathLibrary.BreakVector` (`CharacterMovementComponent.GetLastUpdateVelocity` (`self.CharacterMovement`))))
  (bind _returnvalue (`KismetMathLibrary.Conv_IntToDouble` (`KismetMathLibrary.Round` (`KismetMathLibrary.MapRangeUnclamped` _returnvalue_y 0.0 300.0 0.0 1.0))))
  (bind _returnvalue_2 (`KismetMathLibrary.Conv_IntToDouble` (`KismetMathLibrary.Round` (`KismetMathLibrary.MapRangeUnclamped` _returnvalue_x 0.0 300.0 0.0 1.0))))
  ;[1 1 1] Rotate Enemy to movement direction
  (if (`self.bIsDead`)
    _
    (elif (`self.bIsAttack`)
      _
      (elif (and (`KismetMathLibrary.NearlyEqual_FloatFloat` _returnvalue_2 0.0 0.1) (`KismetMathLibrary.NearlyEqual_FloatFloat` _returnvalue 0.0 0.1))
        (`self.SetAnimMovementDirectionByTarget`)
        (else
          (set `self.MovementDiraction` (`KismetMathLibrary.MakeVector2D` _returnvalue _returnvalue_2)))))))

(event `/Game/UnrealQuest5/Blueprints/Characters/BPI_Character.StartAttack`
  ;[1 0 0 0.5] 攻撃
  (if (not (`self.bIsAttack`))
    (set `self.bIsAttack` true)
    (`self.SetAnimMovementDirectionByTarget`)))

(event `/Game/UnrealQuest5/Blueprints/Characters/BPI_Character.FinishAttack`
  ;[1 0 0 0.5] 攻撃
  (set `self.bIsAttack` false))

(event `ToggleSwordHitBox`
  (params (HiboxSide :type Byte))
  ;[0.1094 0.1094 0.1094] Toggle Swad hitbox. Recievebyta value of hitbox number: 0 - up, 1 - right,  2 - down, 3 - left
  (`SceneComponent.K2_AttachToComponent` (`self.RotationWeaponSocket`) (select `byte` HiboxSide :`0` (`self.SwordN`) :`1` (`self.SwordNE`) :`2` (`self.SwordE`) :`3` (`self.SwordSE`) :`4` (`self.SwordS`) :`5` (`self.SwordSW`) :`6` (`self.SwordW`) :`7` (`self.SwordNW`)) "None" "SnapToTarget" "KeepWorld" "KeepRelative" true)
  (bind _asbp_sword (cast `/Game/UnrealQuest5/Blueprints/Weapons/PlayerWeapon/BP_Sword` (`ChildActorComponent.ChildActor` (`self.Weapon`))))
  (`/Game/UnrealQuest5/Blueprints/Weapons/PlayerWeapon/BP_Sword.SetHitBoxActive` _asbp_sword (not (`/Game/UnrealQuest5/Blueprints/Weapons/PlayerWeapon/BP_Sword.bIsHitBoxActive` _asbp_sword))))

(event `self.ReceiveBeginPlay`
  (bind _returnvalue (`GameplayStatics.GetPlayerCharacter` 0))
  (bind _childactor (`ChildActorComponent.ChildActor` (`self.Weapon`)))
  ;[1 1 1] BeginPlay
  ;;[1 1 1] Set Anim Instance
  (`|ExecutionSequence`
    (:`then_0`
      (message `/Game/UnrealQuest5/Blueprints/Items/BPI_Item.SetTeamNumber` _childactor (`self.TeamNumber`))
      (set `Actor.Instigator` self _childactor))
    (:`then_1`
      ;;[1 1 1] Death Event
      (add `/Game/UnrealQuest5/Blueprints/Components/BPC_HealthComponent.OnDeath` (`self.BPC_HealthComponent`) (delegate `OnDeath_Event`)))
    (:`then_2`
      (bind _returnvalue_2 (`PrimitiveComponent.CreateDynamicMaterialInstance` (`self.Sprite`) 0 "/Game/UnrealQuest5/Materials/MI_EnemyUnlitTranslucentSpriteMaterial.MI_EnemyUnlitTranslucentSpriteMaterial" "None"))
      (set `self.SpriteMaterial` _returnvalue_2))
    (:`then_3`
      ;;[1 1 1] Set Taget Actor
      (`/Engine/EditorBlueprintResources/StandardMacros.IsValid` _returnvalue
        (:`Is Valid`
          (set `self.TargetActor` _returnvalue))))))

(event `OnDeath_Event`
  ;[1 1 1] BeginPlay
  ;;[1 1 1] Death Event
  (set `self.bIsDead` true)
  (`Controller.UnPossess` (`self.GetController`))
  (`ActorComponent.Deactivate` (`self.BPC_HealthComponent`))
  (`PrimitiveComponent.SetCollisionEnabled` (`self.CapsuleComponent`) "NoCollision")
  ;;;[1 1 1] SpawnLoot
  (`self.SpawnLoot`))

(event `self.ReceiveAnyDamage`
  (params (Damage :type "Float (single-precision)") (DamageType :type "DamageType Object Reference") (InstigatedBy :type "Controller Object Reference") (DamageCauser :type "Actor Object Reference"))
  ;[1 1 1] ApplyDamage
  (`parent.ReceiveAnyDamage` Damage DamageType InstigatedBy DamageCauser)
  (if (not (`self.bIsDead`))
    (bind (_direction _alpha) (`Timeline|FlickeringTimeline` :!via `PlayFromStart`)
      (:`Update`
        (`MaterialInstanceDynamic.SetScalarParameterValue` (`self.SpriteMaterial`) "Opacity" (`KismetMathLibrary.Lerp` 2.0 0.5 _alpha))))))

(event `DestroyByTime`
  ;[1 1 1] BeginPlay
  ;;[1 1 1] Destroy by time
  (`Controller.UnPossess` (`self.GetController`))
  (`self.K2_DestroyActor`))

(fn `GetAttackWaitTime`
  (returns (WaitTime :type "Float (double-precision)"))
  (return (`self.AttackWaitTime`)))

(fn `GetBehaviour`
  (returns (BehaviorTree :type "BehaviorTree Object Reference"))
  (return (`self.DefaultBehaviorTree`)))

(fn `GetIsAttack`
  (returns (bIsAttack :type Boolean))
  (return (`self.bIsAttack`)))

(fn `GetMovementDirection`
  (returns (MovementDirection :type "Vector2D Structure"))
  (return (`self.MovementDiraction`)))

(fn `SetAnimMovementDirectionByTarget`
  (bind _returnvalue (`self.K2_GetActorLocation`))
  (bind _returnvalue_2 (`BlackboardComponent.GetValueAsObject` (`AIBlueprintHelperLibrary.GetBlackboard` null) "ChaseActorKey"))
  (bind _targetactor (`self.TargetActor`)
    (:`then`
      _)
    (:`else`
      (`/Engine/EditorBlueprintResources/StandardMacros.IsValid` _returnvalue_2
        (:`Is Valid`
          (bind _asactor (cast `Actor` _returnvalue_2))
          (set `self.TargetActor` _asactor))
        (:`Is Not Valid`
          (set `self.TargetActor` (`GameplayStatics.GetPlayerCharacter` 0))))))
  (bind _returnvalue_3 (`self.K2_GetActorLocation` _targetactor))
  (bind (_returnvalue_x _returnvalue_y) (`KismetMathLibrary.BreakVector` (`KismetMathLibrary.Normal` (- _returnvalue_3 _returnvalue))))
  (set `self.MovementDiraction` (`KismetMathLibrary.MakeVector2D` (`KismetMathLibrary.Conv_IntToDouble` (`KismetMathLibrary.Round` _returnvalue_y)) (`KismetMathLibrary.Conv_IntToDouble` (`KismetMathLibrary.Round` _returnvalue_x))))
  (set `self.LookAtRotation` (`KismetMathLibrary.FindLookAtRotation` (`KismetMathLibrary.MakeVector` (.x _returnvalue) (.y _returnvalue)) (`KismetMathLibrary.MakeVector` (.x _returnvalue_3) (.y _returnvalue_3)))))

(fn `SpawnLoot`
  (bind _returnvalue_location (`KismetMathLibrary.BreakTransform` (`self.GetTransform`)))
  (bind _returnvalue_location_2 (`KismetMathLibrary.BreakTransform` (`self.GetTransform`)))
  (bind _lootclasses (`self.LootClasses`))
  (if (`KismetArrayLibrary.Array_IsNotEmpty` _lootclasses)
    (for _array_element _lootclasses
      (`|SpawnActorFromClass` _array_element (`KismetMathLibrary.MakeTransform` _returnvalue_location_2) "AlwaysSpawn" "OverrideRootScale" self self))
    (if (`KismetMathLibrary.RandomBoolWithWeight` (`self.ChanceToSpawnHeal`))
      (`|SpawnActorFromClass` "/Game/UnrealQuest5/Blueprints/Items/BP_HealItem.BP_HealItem_C" (`KismetMathLibrary.MakeTransform` _returnvalue_location) "AlwaysSpawn" "OverrideRootScale" self self))))

(fn `UserConstructionScript`)