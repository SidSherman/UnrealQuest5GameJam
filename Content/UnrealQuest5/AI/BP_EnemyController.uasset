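; AI controller for enemies that sets up their blackboard and starts their behavior tree to chase the player.
; On BeginPlay it initializes BB_Enemy and, if the player pawn is valid, stores it as the chase target.
; Attack wait time and tree asset come from the controlled BP_EnemyZDCharacter, letting each enemy supply its own behavior.
; The wait time is written to the blackboard before the tree runs.
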(event `self.ReceiveBeginPlay`
  (bind _returnvalue (`GameplayStatics.GetPlayerPawn` 0))
  (bind _blackboardcomponent (`self.UseBlackboard` "/Game/UnrealQuest5/AI/BB_Enemy.BB_Enemy"))
  ;[1 1 1] 敵が追跡するアクターを設定
  (`/Engine/EditorBlueprintResources/StandardMacros.IsValid` _returnvalue
    (:`Is Valid`
      (`BlackboardComponent.SetValueAsObject` _blackboardcomponent "ChaseActorKey" _returnvalue)
      ;[1 1 1] SeT Wait Time
      (bind _asbp_enemy_zdcharacter (cast `/Game/UnrealQuest5/Blueprints/Characters/BP_EnemyZDCharacter` (`self.K2_GetPawn`))
        (:`then`
          (set `self.WaitTime` (`/Game/UnrealQuest5/Blueprints/Characters/BP_EnemyZDCharacter.GetAttackWaitTime` _asbp_enemy_zdcharacter))
          (set `self.BTAsset` (`/Game/UnrealQuest5/Blueprints/Characters/BP_EnemyZDCharacter.GetBehaviour` _asbp_enemy_zdcharacter)))
        (:`CastFailed`
          _))
      ;[1 1 1] 待機時間を設定
      (`BlackboardComponent.SetValueAsFloat` _blackboardcomponent "WaitTimeKey" (`self.WaitTime`))
      ;[1 1 1] ビヘイビアツリーを実行
      (`self.RunBehaviorTree` (`self.BTAsset`)))))

(fn `UserConstructionScript`)