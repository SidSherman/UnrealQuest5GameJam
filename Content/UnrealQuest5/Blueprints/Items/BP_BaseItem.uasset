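; Base item Blueprint with an empty Use event, a cached player character reference, a fixed team number of zero and automatic despawning.
; BeginPlay starts a timer that destroys the item after three minutes unless it gets rendered first.
; Tick watches WasRecentlyRendered: the first sighting cancels that timer, and afterwards the item destroys itself once it has gone unrendered for a minute.
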(event `/Game/UnrealQuest5/Blueprints/Items/BPI_Item.Use`
  (params (Pawn :type "/Game/UnrealQuest5/Blueprints/Characters/BP_PlayerZDCharacter Object Reference")))

(event `self.ReceiveTick`
  (params (DeltaSeconds :type "Float (single-precision)"))
  ;[1 1 1] Destroy if Actor is not rendered for one minute
  (if (`self.bIsRenderedAtOnce`)
    (if (not (`self.WasRecentlyRendered` 60.0))
      (`self.K2_DestroyActor`))
    (elif (`self.WasRecentlyRendered` 1.0)
      (set `self.bIsRenderedAtOnce` true)
      (`KismetSystemLibrary.K2_ClearAndInvalidateTimerHandle` (`self.DestoryTimerHandler`)))))

(event `self.ReceiveBeginPlay`
  (set `self.PlayerRef` (`GameplayStatics.GetPlayerCharacter` 0))
  (bind _returnvalue (`KismetSystemLibrary.K2_SetTimerDelegate` (delegate `DestroyByTime`) 180.0))
  (set `self.DestoryTimerHandler` _returnvalue))

(event `DestroyByTime`
  (`self.K2_DestroyActor`))

(fn `GetTeamNumber`
  (returns (TeamNumber :type Byte))
  (return 0))

(fn `UserConstructionScript`)