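; BP_Bike is a weapon Blueprint that starts shooting automatically on BeginPlay through StartShoot.
; Each Shoot event spawns a Projectile at the root's location, rolled -90 degrees, with yaw randomized within Spreading and scale set by Size.
; The projectile receives the weapon's team number, damage and instigator, and each shot plays a 2D sound.
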(event `self.ReceiveBeginPlay`
  (`parent.ReceiveBeginPlay`)
  (`self.StartShoot`))

(event `self.Shoot`
  (bind _size (`self.Size`))
  (bind _returnvalue (`SceneComponent.K2_GetComponentToWorld` (`self.DefaultSceneRoot`)))
  (`|SpawnActorFromClass` (`self.Projectile`) (`KismetMathLibrary.MakeTransform` (.location _returnvalue) (`KismetMathLibrary.MakeRotator` -90.0 (.pitch (.rotation _returnvalue)) (+ (.yaw (.rotation _returnvalue)) (`KismetMathLibrary.RandomFloatInRange` (* (`self.Spreading`) -1.0) (`self.Spreading`)))) (`KismetMathLibrary.MakeVector` _size _size _size)) "AdjustIfPossibleButAlwaysSpawn" "OverrideRootScale" self (`self.TeamNumber`) (`self.Damage`) (`self.Instigator`))
  (`GameplayStatics.PlaySound2D` null 0.6 1.0 0.0 null null))

(fn `UserConstructionScript`
  (`parent.UserConstructionScript`))