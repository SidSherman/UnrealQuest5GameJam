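; Spawner component that periodically spawns batches of AI or items at random reachable points around its owner, until game over.
; A looping timer fires Spawn, and an optional second timer shortens the interval down to a floor, applied by restarting the spawn timer after the next batch.
; GetRandomPonit retries navmesh points to keep them outside an inner radius, debug-drawing rejects.
; AI spawns and destructions are broadcast through dispatchers.
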(event `self.ReceiveBeginPlay`
  ;[1 1 1] Begin Play
  (set `self.SpawnTime` (`self.DefaultSpawnTime`))
  (bind _asbp_game_state (cast `/Game/UnrealQuest5/Blueprints/General/BP_GameState` (`GameplayStatics.GetGameState`)))
  (add `/Game/UnrealQuest5/Blueprints/General/BP_GameState.OnGameOver` _asbp_game_state (delegate `Stop Spawn`)))

(event `Stop Spawn`
  ;[1 1 1] StopSpawn
  (`KismetSystemLibrary.K2_ClearAndInvalidateTimerHandle` (`self.SpawnTimerHandle`))
  (`KismetSystemLibrary.K2_ClearAndInvalidateTimerHandle` (`self.SpawnTimeDecreasinTimerHandle`))
  (set `self.SpawnTime` (`self.DefaultSpawnTime`)))

(event `StartSpawn`
  (bind _spawntime (`self.SpawnTime`))
  ;[1 1 1] StartSpawn
  (if (`self.bIsFirstSpawn`)
    (`KismetSystemLibrary.Delay` (`self.SpawnDelayDelay`)))
  (bind _returnvalue (`KismetSystemLibrary.K2_SetTimerDelegate` (delegate `Spawn`) _spawntime true (* _spawntime -1.0)))
  (set `self.SpawnTimerHandle` _returnvalue)
  (set `self.bIsFirstSpawn` false)
  (if (`self.bShouldChangeSpawnTime`)
    (if (not (`KismetSystemLibrary.K2_IsValidTimerHandle` (`self.SpawnTimeDecreasinTimerHandle`)))
      (bind _returnvalue_2 (`KismetSystemLibrary.K2_SetTimerDelegate` (delegate `SpawnTimeDecreasing`) (`self.SpawnTimeDecreasingRate`) true))
      (set `self.SpawnTimeDecreasinTimerHandle` _returnvalue_2))))

(event `SpawnTimeDecreasing`
  ;[1 1 1] SpawnTime manager
  (set `self.SpawnTime` (`KismetMathLibrary.FClamp` (- (`self.SpawnTime`) (`self.SpawnTimeDecrement`)) 0.5 10000.0))
  (set `self.bShouldUpdateSpawnTimer` true))

(event `Spawn`
  (bind _outerradius (`self.OuterRadius`))
  (bind (_returnvalue_x _returnvalue_y _returnvalue_z) (`KismetMathLibrary.BreakVector` (`Actor.K2_GetActorLocation` (`self.GetOwner`))))
  (bind _returnvalue (`Actor.K2_GetActorLocation` (`self.GetOwner`)))
  (bind (_randomlocation_x _randomlocation_y) (`KismetMathLibrary.BreakVector` (`self.GetRandomPonit` _returnvalue _outerradius)))
  (bind (_randomlocation_x_2 _randomlocation_y_2) (`KismetMathLibrary.BreakVector` (`self.GetRandomPonit` _returnvalue _outerradius)))
  ;[1 1 1] Spawn
  (for _ (range (`self.Count`))
    (if (`self.bShouldSpawnAI`)
      (bind _returnvalue_2 (`|SpawnActorFromClass` (`self.SpawnAI`) (`KismetMathLibrary.MakeTransform` (`KismetMathLibrary.MakeVector` _randomlocation_x_2 _randomlocation_y_2 _returnvalue_z)) "AdjustIfPossibleButAlwaysSpawn" "OverrideRootScale" null null))
      (`self.SpawnAIDispatcher` _returnvalue_2)
      (add `Actor.OnDestroyed` _returnvalue_2 (delegate `OnDestroyed_Event`))
      (else
        (`|SpawnActorFromClass` (`self.SpawnItem`) (`KismetMathLibrary.MakeTransform` (`KismetMathLibrary.MakeVector` _randomlocation_x _randomlocation_y _returnvalue_z)) "Undefined" "OverrideRootScale" null null))))
  (if (`self.bShouldUpdateSpawnTimer`)
    (set `self.bShouldUpdateSpawnTimer` false)
    (`KismetSystemLibrary.K2_ClearAndInvalidateTimerHandle` (`self.SpawnTimerHandle`))
    (`self.StartSpawn`)))

(event `OnDestroyed_Event`
  (params (DestroyedActor :type "Actor Object Reference"))
  ;[1 1 1] Spawn
  (`self.OnAIDestroy` DestroyedActor))

(fn `GetRandomPonit`
  (params (Origin :type "Vector Structure (by ref)") (Radius :type "Float (single-precision)"))
  (returns (RandomLocation :type "Vector Structure"))
  (locals (RandLocation :type "Vector Structure" :default (0.0 0.0 0.0)))
  (bind _randlocation (`local.RandLocation`))
  (for _ (range (+ (`self.MaxIteration`) 1))
    (bind _output_get (set `local.RandLocation` (`NavigationSystemV1.K2_GetRandomReachablePointInRadius` Origin Radius null null)))
    (if (> (`KismetMathLibrary.Vector_Distance2D` _output_get (`local.Origin`)) (`self.InnerRadius`))
      (return _randlocation)
      (else
        (`KismetSystemLibrary.DrawDebugSphere` _randlocation 100.0 12 (struct :`R` 1.0 :`G` 1.0 :`B` 1.0 :`A` 1.0) 5.0))))
  (return (`local.RandLocation`)))