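; BP_HP is a weapon-slot upgrade that regenerates and raises its owner's health instead of attacking.
; StartShoot runs a looping one-second timer on Shoot, which heals through the owner's BPC_HealthComponent by passing negated Damage until health is full.
; IncreaseHP repurposes the Size stat to adjust max health, and events re-fetch the component if the cached reference is invalid.
; SpetialSkill is empty, and IncreaseHealsCount only refreshes that reference.
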(event `self.ReceiveBeginPlay`
  ;[1 1 1] Begin Play
  (`parent.ReceiveBeginPlay`)
  (set `self.HealthComponent` (`self.GetComponentByClass` (`self.GetOwner`) "/Game/UnrealQuest5/Blueprints/Components/BPC_HealthComponent.BPC_HealthComponent_C")))

(event `/Game/_HentaiShooter/Weapons/BPI_Weapon.StartShoot`
  ;[1 1 1] Start Recover HP
  (bind _returnvalue (`KismetSystemLibrary.K2_SetTimerDelegate` (delegate `/Game/_HentaiShooter/Weapons/BPI_Weapon.Shoot`) 1.0 true))
  (set `self.ShootingTimer` _returnvalue))

(event `/Game/_HentaiShooter/Weapons/BPI_Weapon.Shoot`
  (bind _returnvalue (`self.GetComponentByClass` (`self.GetOwner`) "/Game/UnrealQuest5/Blueprints/Components/BPC_HealthComponent.BPC_HealthComponent_C"))
  ;[1 1 1] Recover HP
  (`self.HealthComponent`
    (:`then`
      _)
    (:`else`
      (`/Engine/EditorBlueprintResources/StandardMacros.IsValid` _returnvalue
        (:`Is Valid`
          (bind _output_get (set `self.HealthComponent` _returnvalue))))))
  (if (not (`/Game/UnrealQuest5/Blueprints/Components/BPC_HealthComponent.bIsMaxHealth` _output_get))
    (`/Game/UnrealQuest5/Blueprints/Components/BPC_HealthComponent.CalculateHealth` _output_get (* (`self.Damage`) -1.0))))

(event `IncreaseHealsCount`
  (bind _returnvalue (`self.GetComponentByClass` (`self.GetOwner`) "/Game/UnrealQuest5/Blueprints/Components/BPC_HealthComponent.BPC_HealthComponent_C"))
  (`self.HealthComponent`
    (:`then`)
    (:`else`
      (`/Engine/EditorBlueprintResources/StandardMacros.IsValid` _returnvalue
        (:`Is Valid`
          (set `self.HealthComponent` _returnvalue))))))

(event `IncreaseHP`
  (bind _returnvalue (`self.GetComponentByClass` (`self.GetOwner`) "/Game/UnrealQuest5/Blueprints/Components/BPC_HealthComponent.BPC_HealthComponent_C"))
  ;[1 1 1] Increase HP
  (`self.HealthComponent`
    (:`then`
      _)
    (:`else`
      (`/Engine/EditorBlueprintResources/StandardMacros.IsValid` _returnvalue
        (:`Is Valid`
          (bind _output_get (set `self.HealthComponent` _returnvalue))))))
  (`/Game/UnrealQuest5/Blueprints/Components/BPC_HealthComponent.SetMaxHealth` _output_get (- (`self.Size`) (`/Game/UnrealQuest5/Blueprints/Components/BPC_HealthComponent.MaxHealth` _output_get))))

(event `/Game/_HentaiShooter/Weapons/BPI_Weapon.SpetialSkill`)

(fn `UserConstructionScript`
  (`parent.UserConstructionScript`))