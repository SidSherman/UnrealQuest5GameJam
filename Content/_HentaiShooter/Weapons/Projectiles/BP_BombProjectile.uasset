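; Bomb projectile that deals area damage and spawns an explosion when destroyed, building on a parent projectile class.
; On destruction it plays a sound, damages every BP_ZDBaseCharacter overlapping its capsule, and spawns explosion FX scaled by its size.
; A one-shot timer after MoveTime applies a single interpolation step reducing Speed toward zero.
; Its ActorBeginOverlap event is empty, so this graph deals damage only on destruction.
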(event `self.ReceiveBeginPlay`
  (`parent.ReceiveBeginPlay`)
  (bind _returnvalue (`KismetSystemLibrary.K2_SetTimerDelegate` (delegate `StopMove`) (`self.MoveTime`)))
  (set `self.MovementTimerHandle` _returnvalue)
  (add `self.OnDestroyed` (delegate `OnDestroyed_Event`)))

(event `OnDestroyed_Event` :!signature `self.OnDestroyed`
  (params (DestroyedActor :type "Actor Object Reference"))
  (bind (_returnvalue_location _returnvalue_rotation) (`KismetMathLibrary.BreakTransform` (`self.GetTransform`)))
  (bind (_returnvalue_location_2 _returnvalue_rotation_2) (`KismetMathLibrary.BreakTransform` (`self.GetTransform`)))
  (`GameplayStatics.PlaySoundAtLocation` "/Engine/VREditor/Sounds/UI/Camera_Shutter.Camera_Shutter" _returnvalue_location _returnvalue_rotation 1.0 1.0 0.0 null null DestroyedActor null)
  (for _array_element (`PrimitiveComponent.GetOverlappingActors` (`self.Capsule`) "/Game/_HentaiShooter/Characters/BP_ZDBaseCharacter.BP_ZDBaseCharacter_C")
    (`KismetSystemLibrary.PrintString` (`KismetSystemLibrary.GetDisplayName` _array_element))
    (`self.Damage Actor` _array_element))
  (`|SpawnActorFromClass` (`self.ExplosionFX`) (`KismetMathLibrary.MakeTransform` _returnvalue_location_2 _returnvalue_rotation_2 (* (`self.ExplosionScale`) (`self.Size`))) "AlwaysSpawn" "OverrideRootScale" null null))

(event `StopMove`
  (set `self.Speed` (`KismetMathLibrary.FInterpTo` (`self.Speed`) 0.0 (`GameplayStatics.GetWorldDeltaSeconds`) (/ (`self.Speed`) 5.0))))

(event `self.ReceiveActorBeginOverlap`
  (params (OtherActor :type "Actor Object Reference")))

(fn `UserConstructionScript`
  (`parent.UserConstructionScript`))