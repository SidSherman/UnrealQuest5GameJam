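; BP_BaseItem is a base item Blueprint with an empty Use event and a GetTeamNumber function that returns a neutral-looking zero.
; On BeginPlay it caches the player character.
; Every Tick it measures its distance to that player and destroys itself once more than 10000 units away.
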(event `/Game/UnrealQuest5/Blueprints/Weapons/BPI_Item.Use`
  (params (Pawn :type "/Game/UnrealQuest5/Blueprints/Characters/BP_PlayerZDCharacter Object Reference")))

(event `self.ReceiveBeginPlay`
  (set `self.PlayerRef` (`GameplayStatics.GetPlayerCharacter` 0)))

(event `self.ReceiveTick`
  (params (DeltaSeconds :type "Float (single-precision)"))
  (bind _playerref (`self.PlayerRef`)
    (:`then`
      (if (> (`KismetMathLibrary.Vector_Distance` (`self.K2_GetActorLocation` _playerref) (`self.K2_GetActorLocation`)) 10000.0)
        (`self.K2_DestroyActor`)))
    (:`else`)))

(fn `GetTeamNumber`
  (returns (TeamNumber :type Byte))
  (return 0))

(fn `UserConstructionScript`)