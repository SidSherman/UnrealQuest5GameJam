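; BP_BaseCharacter is a base character Blueprint that provides health and team membership.
; Incoming AnyDamage is forwarded to its health component, and BeginPlay caches a reference to BP_GameState.
; It stores a team number through SetTeamNumber and returns it through GetTeamNumber.
; The attack, movement and direction getters are stubs returning false or a zero vector.
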(event `self.ReceiveAnyDamage`
  (params (Damage :type "Float (single-precision)") (DamageType :type "DamageType Object Reference") (InstigatedBy :type "Controller Object Reference") (DamageCauser :type "Actor Object Reference"))
  (`/Game/UnrealQuest5/Blueprints/Components/BPC_HealthComponent.CalculateHealth` (`self.BPC_HealthComponent`) Damage))

(event `self.ReceiveBeginPlay`
  (bind _asbp_game_state (cast `/Game/UnrealQuest5/Blueprints/General/BP_GameState` (`GameplayStatics.GetGameState`)))
  (set `self.BP Game State` _asbp_game_state))

(event `/Game/UnrealQuest5/Blueprints/Weapons/BPI_Item.SetTeamNumber`
  (params (TeamNumber :type Byte))
  (set `self.TeamNumber` TeamNumber))

(fn `GetIsAttack`
  (returns (bIsAttack :type Boolean))
  (return false))

(fn `GetIsMove`
  (returns (bIsMove :type Boolean))
  (return false))

(fn `GetMovementDirection`
  (returns (MovementDirection :type "Vector2D Structure"))
  (return (0.0 0.0)))

(fn `GetTeamNumber`
  (returns (TeamNumber :type Byte))
  (return (`self.TeamNumber`)))

(fn `UserConstructionScript`)