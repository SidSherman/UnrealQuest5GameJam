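; BP_Fist is a melee fist weapon that deals damage through a briefly activated hitbox.
; StartShoot runs a looping timer scaled by global time dilation, using a negative start delay to cancel the first wait.
; Each Shoot resizes the hitbox by Size, enables query collision and shows the flipbook until a second timer reverts both collision and visibility.
; Overlaps damage any actor except the Instigator, crediting its controller.
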(event `self.ReceiveBeginPlay`
  (`parent.ReceiveBeginPlay`)
  (set `self.DefaultHitBoxSize` (`BoxComponent.GetUnscaledBoxExtent` (`self.HitBox`))))

(event `/Game/_HentaiShooter/Weapons/BPI_Weapon.StartShoot`
  (bind _shootingrate (`self.ShootingRate`))
  (`KismetSystemLibrary.K2_ClearAndInvalidateTimerHandle` (`self.ShootingTimer`))
  (`KismetSystemLibrary.K2_ClearAndInvalidateTimerHandle` (`self.ActivateTimerHandle`))
  (bind _returnvalue (`KismetSystemLibrary.K2_SetTimerDelegate` (delegate `/Game/_HentaiShooter/Weapons/BPI_Weapon.Shoot`) (* _shootingrate (`GameplayStatics.GetGlobalTimeDilation`)) true (* (* _shootingrate -1.0) (`GameplayStatics.GetGlobalTimeDilation`))))
  (set `self.ShootingTimer` _returnvalue))

(event `/Game/_HentaiShooter/Weapons/BPI_Weapon.Shoot`
  (`BoxComponent.SetBoxExtent` (`self.HitBox`) (* (`self.DefaultHitBoxSize`) (`self.Size`)) true)
  (set `self.bIsHitActive` true)
  (`SceneComponent.SetHiddenInGame` (`self.PaperFlipbook`) false false)
  (`PrimitiveComponent.SetCollisionEnabled` (`self.HitBox`) "QueryOnly")
  (bind _returnvalue (`KismetSystemLibrary.K2_SetTimerDelegate` (delegate `/Game/_HentaiShooter/Weapons/BPI_Weapon.StopShoot`) (`self.ActiveTime`)))
  (set `self.ActivateTimerHandle` _returnvalue))

(event `/Game/_HentaiShooter/Weapons/BPI_Weapon.StopShoot`
  (`PrimitiveComponent.SetCollisionEnabled` (`self.HitBox`) "NoCollision")
  (`SceneComponent.SetHiddenInGame` (`self.PaperFlipbook`) true false)
  (set `self.bIsHitActive` false))

(event `self.HitBox.OnComponentBeginOverlap`
  (params (OverlappedComponent :type "PrimitiveComponent Object Reference") (OtherActor :type "Actor Object Reference") (OtherComp :type "PrimitiveComponent Object Reference") (OtherBodyIndex :type Integer) (bFromSweep :type Boolean) (SweepResult :type "HitResult Structure (by ref)"))
  (bind _instigator (`self.Instigator`))
  (`/Engine/EditorBlueprintResources/StandardMacros.IsValid` _instigator
    (:`Is Valid`
      (if (!= OtherActor _instigator)
        (`GameplayStatics.ApplyDamage` OtherActor (`self.Damage`) (`Pawn.GetController` _instigator) self "/Script/Engine.DamageType")))))

(fn `UserConstructionScript`
  (`parent.UserConstructionScript`))