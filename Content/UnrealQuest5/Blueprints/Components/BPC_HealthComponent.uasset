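; BPC_HealthComponent is a health component that tracks current and maximum health for its owner, starting at full health on BeginPlay.
; CalculateHealth subtracts damage, clamps the result between zero and the maximum, then fires OnHealthChanged, plus OnDeath at zero.
; IncreaseHealth adds a capped, non-negative amount to maximum health and heals by that amount, passing it to CalculateHealth as negative damage.
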(event `self.ReceiveBeginPlay`
  (set `self.CurrentHealth` (`self.MaxHealth`)))

(event `CalculateHealth`
  (params (Damage :type "Float (double-precision)"))
  (bind _output_get (set `self.CurrentHealth` (`KismetMathLibrary.FClamp` (- (`self.CurrentHealth`) Damage) 0.0 (`self.MaxHealth`))))
  (`self.OnHealthChanged`)
  (if (<= _output_get 0.0)
    (`self.OnDeath`)))

(event `IncreaseHealth`
  (params (Health :type "Float (double-precision)"))
  (bind _returnvalue (`KismetMathLibrary.FClamp` Health 0.0 1000.0))
  (set `self.MaxHealth` (+ _returnvalue (`self.MaxHealth`)))
  (`self.CalculateHealth` (* _returnvalue -1.0)))