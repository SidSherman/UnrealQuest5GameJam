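; BP_Sword is a melee weapon that damages actors overlapping its box hitbox while that hitbox is active.
; Each tick during the active window, it polls the box overlaps and applies damage to actors whose team number, read via a message call, differs from its own.
; An array of already-hit actors limits damage to once per activation and is cleared whenever SetHitBoxActive is called.
; The construction script sizes the box from HitboxSize.
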(event `self.ReceiveTick`
  (params (DeltaSeconds :type "Float (single-precision)"))
  (if (`self.bIsHitBoxActive`)
    (`self.CheckHit`)))

(event `CheckHit`
  (bind _output_get (set `self.Overlapping Actors` (`PrimitiveComponent.GetOverlappingActors` (`self.Box`) null)))
  (if (`KismetArrayLibrary.Array_IsNotEmpty` _output_get)
    (for _array_element (`self.Overlapping Actors`)
      (bind _team (message `/Game/UnrealQuest5/Blueprints/Characters/BPI_Character.GetTeamNumber` _array_element))
      (if (and (!= _team (`self.TeamNumber`)) (not (`KismetArrayLibrary.Array_Contains` (`self.DamagedForHitThisActor`) _array_element)))
        (`GameplayStatics.ApplyDamage` _array_element (`self.Damage`) null self)
        (`KismetArrayLibrary.Array_AddUnique` (`self.DamagedForHitThisActor`) _array_element)))))

(fn `GetHitBoxActive`
  (returns (bIsHitBoxActive :type Boolean))
  (return (`self.bIsHitBoxActive`)))

(fn `SetHitBoxActive`
  (params (bIsHitBoxActive :type Boolean))
  (set `self.bIsHitBoxActive` bIsHitBoxActive)
  (`KismetArrayLibrary.Array_Clear` (`self.DamagedForHitThisActor`)))

(fn `UserConstructionScript`
  (`parent.UserConstructionScript`)
  (`BoxComponent.SetBoxExtent` (`self.Box`) (`self.HitboxSize`) true))