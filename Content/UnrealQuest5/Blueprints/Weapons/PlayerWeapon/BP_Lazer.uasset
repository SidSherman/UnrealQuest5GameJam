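; Player laser weapon that starts shooting on BeginPlay and fires beams in random directions, damaging objects along their paths.
; Each recursive LineTrace step applies damage through a debug-drawn, Size-scaled multi-sphere trace over a fixed range, skipping the instigator's pawn.
; A visibility trace then bounces the beam off surfaces via a flattened reflection vector, or continues from the trace end on a miss, until ProjectileCount segments are reached.
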(event `self.ReceiveBeginPlay`
  (`parent.ReceiveBeginPlay`)
  (`self.StartShoot`))

(event `self.Shoot`
  (set `self.CurrentProjectileCount` 0)
  (`self.LineTrace` (`KismetMathLibrary.MakeVector` (* (`KismetMathLibrary.RandomFloat`) (`KismetMathLibrary.SelectInt` 1 -1 (`KismetMathLibrary.RandomBool`))) (* (`KismetMathLibrary.RandomFloat`) (`KismetMathLibrary.SelectInt` 1 -1 (`KismetMathLibrary.RandomBool`)))) (`SceneComponent.K2_GetComponentLocation` (`self.DefaultSceneRoot`)) null (`self.Size`)))

(fn `GetReflectionVector`
  (params (Direction :type "Vector Structure") (SurfaceNormal :type "Vector Structure"))
  (returns (ReturnValue :type "Vector Structure"))
  (return (`KismetMathLibrary.GetForwardVector` (`KismetMathLibrary.MakeRotFromX` (`KismetMathLibrary.Vector_Normal2D` (`KismetMathLibrary.GetReflectionVector` Direction SurfaceNormal))))))

(fn `LineTrace`
  (params (Direction :type "Vector Structure") (Location :type "Vector Structure") (IgnoredActor :type "Actor Object Reference") (Size :type "Float (double-precision)"))
  (bind _returnvalue (`self.GetInstigatorController`))
  (bind (_outhits _returnvalue_2) (`KismetSystemLibrary.SphereTraceMultiForObjects` :`Start` Location :`End` (+ Location (* Direction 3000.0)) :`Radius` (* Size (`self.DefaultRadius`)) :`ObjectTypes` (`|MakeArray` "ObjectTypeQuery8" :!type "EObjectTypeQuery Enum") :`DrawDebugType` "ForDuration" :`DrawTime` 0.5))
  (if _returnvalue_2
    (for _array_element _outhits
      (if (!= (`.HitActor` (`GameplayStatics.BreakHitResult` _array_element)) (`Controller.K2_GetPawn` _returnvalue))
        (`GameplayStatics.ApplyDamage` (`.HitActor` (`GameplayStatics.BreakHitResult` _array_element)) (`self.Damage`) _returnvalue self))))
  (bind _result (`/Engine/EditorBlueprintResources/StandardMacros.IncrementInt` (`self.CurrentProjectileCount`))
    (:`  `
      (`KismetSystemLibrary.PrintString` (`KismetStringLibrary.Conv_IntToString` _result))
      (bind (_outhit _returnvalue_3) (`KismetSystemLibrary.LineTraceSingle` Location (+ Location (* Direction 3000.0)) "TraceTypeQuery1" true (`|MakeArray` IgnoredActor) "None" true (struct :`R` 1.0 :`A` 1.0) (struct :`G` 1.0 :`A` 1.0) (`self.ShootingRate`)))
      (if (>= (`self.CurrentProjectileCount`) (`self.ProjectileCount`))
        _
        (elif _returnvalue_3
          (bind (_bblockinghit _binitialoverlap _time _distance _location _impactpoint _normal _impactnormal _physmat _hitactor _hitcomponent _hitbonename _bonename _hititem _elementindex _faceindex _tracestart _traceend) (`GameplayStatics.BreakHitResult` _outhit))
          (`self.LineTrace` (`self.GetReflectionVector` Direction _normal) _location _hitactor Size)
          (else
            (`self.LineTrace` (`KismetMathLibrary.GreaterGreater_VectorRotator` _traceend (struct :`Yaw` 90.0)) _traceend _hitactor Size)))))))

(fn `UserConstructionScript`
  (`parent.UserConstructionScript`))