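; BP_TotemSpawner is a spawner that places totems at random positions on BeginPlay and watches for their destruction.
; SpawnTotems creates BP_TotemPlace actors, currently one, using the Box's extents around world origin for X/Y and the player character's height for Z.
; It binds to each place's child TotemActor OnDestroyed, whose handler removes it from the Totems array and prints debug messages, including when none remain.
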(event `self.ReceiveBeginPlay`
  (`self.SpawnTotems` 1))

(event `SpawnTotems`
  (params (Count :type Integer))
  (bind (_returnvalue_x _returnvalue_y) (`KismetMathLibrary.BreakVector` (`BoxComponent.GetScaledBoxExtent` (`self.Box`))))
  (bind (_returnvalue_x_2 _returnvalue_y_2 _returnvalue_z) (`KismetMathLibrary.BreakVector` (`self.K2_GetActorLocation` (`GameplayStatics.GetPlayerCharacter` 0))))
  (for _ (range Count)
    (bind _returnvalue (`|SpawnActorFromClass` "/Game/UnrealQuest5/Blueprints/Characters/Enemies/BP_TotemPlace.BP_TotemPlace_C" (`KismetMathLibrary.MakeTransform` (`KismetMathLibrary.MakeVector` (`KismetMathLibrary.RandomFloatInRange` (* _returnvalue_x -1.0) _returnvalue_x) (`KismetMathLibrary.RandomFloatInRange` (* _returnvalue_y -1.0) _returnvalue_y) _returnvalue_z)) "Undefined" "OverrideRootScale" null null))
    (add `self.OnDestroyed` (`ChildActorComponent.ChildActor` (`/Game/UnrealQuest5/Blueprints/Characters/Enemies/BP_TotemPlace.TotemActor` _returnvalue)) (delegate `OnDestroyed_Event`))
    (`KismetArrayLibrary.Array_AddUnique` (`self.Totems`))))

(event `OnDestroyed_Event` :!signature `self.OnDestroyed`
  (params (DestroyedActor :type "Actor Object Reference"))
  (`KismetSystemLibrary.PrintString` "Totem destroy")
  (`KismetArrayLibrary.Array_RemoveItem` (`self.Totems`) DestroyedActor)
  (if (`KismetArrayLibrary.Array_IsEmpty` (`self.Totems`))
    (`KismetSystemLibrary.PrintString` "All totems removed")))

(fn `UserConstructionScript`)