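; Melee sword weapon Blueprint that damages other-team actors overlapping its box hitbox.
; SetHitBoxActive toggles hitbox collision and a flag that makes Tick call Shoot, which applies damage once per actor via a hit list cleared on deactivation.
; StartShoot also enables the hitbox and starts a looping Shoot timer at the shooting rate.
; The construction script sizes the box from HitboxSize.
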(event `self.ReceiveBeginPlay`
  (`parent.ReceiveBeginPlay`))

(event `self.ReceiveTick`
  (params (DeltaSeconds :type "Float (single-precision)"))
  ;[1 1 1] ApplyDamage
  (if (`self.bIsHitBoxActive`)
    (`/Game/UnrealQuest5/Blueprints/Weapons/BPI_Weapon.Shoot`)))

(event `/Game/UnrealQuest5/Blueprints/Weapons/BPI_Weapon.StartShoot`
  (bind _shootingrate (`self.ShootingRate`))
  ;[1 1 1] Start Shoot
  (bind _returnvalue (`KismetSystemLibrary.K2_SetTimerDelegate` (delegate `/Game/UnrealQuest5/Blueprints/Weapons/BPI_Weapon.Shoot`) _shootingrate true 0.0 (* _shootingrate -1.0)))
  (set `self.ShootingTimeHandle` _returnvalue)
  (`PrimitiveComponent.SetCollisionEnabled` (`self.HitBox`) "QueryOnly"))

(event `/Game/UnrealQuest5/Blueprints/Weapons/BPI_Weapon.Shoot`
  ;[1 1 1] Apply Damage
  (bind _output_get (set `self.Overlapping Actors` (`PrimitiveComponent.GetOverlappingActors` (`self.HitBox`) null)))
  (if (`KismetArrayLibrary.Array_IsNotEmpty` _output_get)
    (for _array_element (`self.Overlapping Actors`)
      (bind _teamnumber (message `/Game/UnrealQuest5/Blueprints/Items/BPI_Item.GetTeamNumber` _array_element))
      (if (and (!= _teamnumber (`self.TeamNumber`)) (not (`KismetArrayLibrary.Array_Contains` (`self.DamagedForHitThisActor`) _array_element)))
        (`GameplayStatics.ApplyDamage` _array_element (`self.Damage`) null self)
        (`KismetArrayLibrary.Array_AddUnique` (`self.DamagedForHitThisActor`) _array_element)))))

(fn `GetHitBoxActive`
  (returns (bIsHitBoxActive :type Boolean))
  (return (`self.bIsHitBoxActive`)))

(fn `SetHitBoxActive`
  (params (bIsHitBoxActive :type Boolean))
  (bind _output_get (set `self.bIsHitBoxActive` bIsHitBoxActive))
  (if _output_get
    (`PrimitiveComponent.SetCollisionEnabled` (`self.HitBox`) "QueryOnly")
    (else
      (`KismetArrayLibrary.Array_Clear` (`self.DamagedForHitThisActor`))
      (`PrimitiveComponent.SetCollisionEnabled` (`self.HitBox`) "NoCollision"))))

(fn `UserConstructionScript`
  (`parent.UserConstructionScript`)
  (`BoxComponent.SetBoxExtent` (`self.HitBox`) (`self.HitboxSize`) true))