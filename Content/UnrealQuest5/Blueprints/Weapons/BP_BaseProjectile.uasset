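; Base projectile actor that flies straight ahead and damages overlapped actors on a different team.
; Tick moves it along its forward vector by Speed with a swept offset, and BeginPlay limits its life span to Lifetime.
; On overlap it queries the other actor's team number by message, applies Damage if the teams differ, then calls the OnHit dispatcher, whose bound handler is empty here.
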(event `self.ReceiveBeginPlay`
  (add `self.OnHit` (delegate `OnHit_Event`))
  (`self.SetLifeSpan` (`self.Lifetime`)))

(event `OnHit_Event`)

(event `self.ReceiveActorBeginOverlap`
  (params (OtherActor :type "Actor Object Reference"))
  (bind _team (message `/Game/UnrealQuest5/Blueprints/Characters/BPI_Character.GetTeamNumber` OtherActor))
  (if (!= _team (`self.TeamNumber`))
    (`GameplayStatics.ApplyDamage` OtherActor (`self.Damage`) null self)
    (`self.OnHit`)))

(event `self.ReceiveTick`
  (params (DeltaSeconds :type "Float (single-precision)"))
  (`self.K2_AddActorWorldOffset` (* (`self.GetActorForwardVector`) (* DeltaSeconds (`self.Speed`))) true))

(fn `UserConstructionScript`)