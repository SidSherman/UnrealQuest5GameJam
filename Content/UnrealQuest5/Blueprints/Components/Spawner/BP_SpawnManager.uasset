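; Spawn manager component that starts timed spawning of enemies, heal items and point items at BeginPlay, each behind its own toggle.
; It adds one BP_SpawnComponent to its owner per enemy type from a data table row, plus one each for heals and points with hardcoded timings.
; It tracks live enemies through spawn and destroy dispatchers, so a time dilation change applies to existing and newly spawned enemies.
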(event `self.ReceiveBeginPlay`
  ;[1 1 1] Start Spawn
  (bind _asbp_game_state (cast `/Game/UnrealQuest5/Blueprints/General/BP_GameState` (`GameplayStatics.GetGameState`)))
  (set `self.GameState` _asbp_game_state)
  (`self.StartSpawn`))

(event `StartSpawn`
  (`|ExecutionSequence`
    (:`then_0`
      ;[1 1 1] Start Spawn Enemies
      (if (`self.bShouldSpawnEnemies`)
        (bind _returnvalue (`|GetDataTableRow` (`self.EnemiesDataBase`) "DefalutValues")
          (:`then`
            (bind (_enemy _count _defaultspawntime _spawntimedecrement _spawntimedecreasingrate _spawndelay) (break `/Game/UnrealQuest5/Blueprints/Components/Spawner/EnemiesSpawn_struct` _returnvalue))
            (if (`KismetArrayLibrary.Array_IsNotEmpty` _enemy)
              (for (_array_element _array_index) _enemy
                (bind _returnvalue_2 (`|AddComponentByClass` (`self.GetOwner`) "/Game/UnrealQuest5/Blueprints/Components/Spawner/BP_SpawnComponent.BP_SpawnComponent_C" _array_element null (`|GetArrayItem` _defaultspawntime _array_index) (`|GetArrayItem` _spawntimedecrement _array_index) (`|GetArrayItem` _spawntimedecreasingrate) (`|GetArrayItem` _count _array_index) true (`|GetArrayItem` _spawndelay _array_index) (`self.GameState`)))
                (`/Game/UnrealQuest5/Blueprints/Components/Spawner/BP_SpawnComponent.StartSpawn` _returnvalue_2)
                (add `/Game/UnrealQuest5/Blueprints/Components/Spawner/BP_SpawnComponent.OnAIDestroy` _returnvalue_2 (delegate `OnAIDestroy_Event`))
                (add `/Game/UnrealQuest5/Blueprints/Components/Spawner/BP_SpawnComponent.SpawnAIDispatcher` _returnvalue_2 (delegate `SpawnAIDispatcher_Event`))))))))
    (:`then_1`
      ;[1 1 1] Spawn Heals
      (if (`self.bShouldSpawnHeals`)
        (bind _returnvalue_3 (`|AddComponentByClass` (`self.GetOwner`) "/Game/UnrealQuest5/Blueprints/Components/Spawner/BP_SpawnComponent.BP_SpawnComponent_C" null "/Game/_HentaiShooter/Items/BP_HealItem.BP_HealItem_C" 25.0 0.0 30.0 1 false 25.0 (`self.GameState`)))
        (`/Game/UnrealQuest5/Blueprints/Components/Spawner/BP_SpawnComponent.StartSpawn` _returnvalue_3)))
    (:`then_2`
      ;[1 1 1] Spawn Score
      (if (`self.bShouldSpawnPoints`)
        (bind _returnvalue_4 (`|AddComponentByClass` (`self.GetOwner`) "/Game/UnrealQuest5/Blueprints/Components/Spawner/BP_SpawnComponent.BP_SpawnComponent_C" null "/Game/_HentaiShooter/Items/PointItems/BP_PointItem.BP_PointItem_C" 2.0 0.0 10.0 1 false 0.0 (`self.GameState`)))
        (`/Game/UnrealQuest5/Blueprints/Components/Spawner/BP_SpawnComponent.StartSpawn` _returnvalue_4)))))

(event `SpawnAIDispatcher_Event`
  (params (AI :type "Pawn Object Reference"))
  ;[1 1 1] Start Spawn Enemies
  (`KismetArrayLibrary.Array_AddUnique` (`self.Enemies`) AI)
  (set `Actor.CustomTimeDilation` (`self.CurrentEnemiesTimeDilation`) AI))

(event `OnAIDestroy_Event`
  (params (Pawn :type "Actor Object Reference"))
  ;[1 1 1] Start Spawn Enemies
  (`KismetArrayLibrary.Array_RemoveItem` (`self.Enemies`) Pawn))

(event `SetEnemiesTimeDilation`
  (params (NewTimeDilation :type "Float (double-precision)"))
  ;[1 1 1] Set AI TIme Dilation
  (bind _output_get (set `self.CurrentEnemiesTimeDilation` NewTimeDilation))
  (for _array_element (`self.Enemies`)
    (set `Actor.CustomTimeDilation` _output_get _array_element)))