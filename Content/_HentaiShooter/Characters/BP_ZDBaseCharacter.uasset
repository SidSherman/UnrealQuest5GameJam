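; Base character that provides a timed dash, damage intake and weapon equipping.
; Dash stores the current move axes, multiplies walk speed and ignores a custom collision channel, then timers restore both and gate a recharge.
; EquipWeapon spawns the class, switches on its type to register it with the weapon component, and attaches it to that type's socket.
; AnyDamage feeds the health component, which the HP weapon also receives.
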(event `Dash`
  (bind _charactermovement (`self.CharacterMovement`))
  ;[1 1 1] Dash Logic
  (if (and (not (`KismetSystemLibrary.K2_IsValidTimerHandle` (`self.DashRechargeTimerHAndler`))) (not (`KismetSystemLibrary.K2_IsValidTimerHandle` (`self.DashTimerHandler`))))
    (set `self.bShouldDash` true)
    (set `CharacterMovementComponent.MaxWalkSpeed` (* (`CharacterMovementComponent.MaxWalkSpeed` _charactermovement) (`self.DashSpeedMultiplicator`)) _charactermovement)
    (`self.SetDashForwardAxis`)
    (`self.SetDashRightAxis`)
    (`PrimitiveComponent.SetCollisionResponseToChannel` (`self.CapsuleComponent`) "ECC_GameTraceChannel2" "ECR_Ignore")
    (bind _returnvalue (`KismetSystemLibrary.K2_SetTimerDelegate` (delegate `StopDash`) (`self.DashTime`)))
    (set `self.DashTimerHandler` _returnvalue)))

(event `StopDash`
  (bind _charactermovement (`self.CharacterMovement`))
  ;[1 1 1] Dash Logic
  (set `self.bShouldDash` false)
  (`KismetSystemLibrary.K2_ClearAndInvalidateTimerHandle` (`self.DashTimerHandler`))
  (set `CharacterMovementComponent.MaxWalkSpeed` (/ (`CharacterMovementComponent.MaxWalkSpeed` _charactermovement) (`self.DashSpeedMultiplicator`)) _charactermovement)
  (`PrimitiveComponent.SetCollisionResponseToChannel` (`self.CapsuleComponent`) "ECC_GameTraceChannel2" "ECR_Block")
  (bind _returnvalue (`KismetSystemLibrary.K2_SetTimerDelegate` (delegate `DashRecharge`) (`self.DashRechargeTime`)))
  (set `self.DashRechargeTimerHAndler` _returnvalue))

(event `DashRecharge`
  ;[1 1 1] Dash Logic
  (`KismetSystemLibrary.K2_ClearAndInvalidateTimerHandle` (`self.DashRechargeTimerHAndler`)))

(event `self.ReceiveTick`
  (params (DeltaSeconds :type "Float (single-precision)"))
  ;[1 1 1] Tick
)

(event `self.ReceiveAnyDamage`
  (params (Damage :type "Float (single-precision)") (DamageType :type "DamageType Object Reference") (InstigatedBy :type "Controller Object Reference") (DamageCauser :type "Actor Object Reference"))
  ;[1 1 1] Begin Play
  (`/Game/_HentaiShooter/Characters/BP_HealthComponent.CalculateHealth` (`self.BP_HealthComponent`) Damage))

(event `self.ReceiveBeginPlay`
  ;[1 1 1] Begin Play
  (bind _asbp_game_state (cast `/Game/_HentaiShooter/Core/BP_GameState` (`GameplayStatics.GetGameState`))
    (:`then`
      (set `self.GameStateRef` _asbp_game_state))
    (:`CastFailed`
      _))
  (set `self.DefaultSpriteScale` (`SceneComponent.RelativeScale3D` (`self.Sprite`))))

(event `EquipWeapon`
  (params (WeaponClass :type "/Game/_HentaiShooter/Weapons/Weapons/BP_BaseWeapon Class Reference"))
  (bind _weaponsocketposition (`self.WeaponSocketPosition`))
  ;[1 1 1] EquipWeapon
  (bind _returnvalue (`|SpawnActorFromClass` WeaponClass (`SceneComponent.K2_GetComponentToWorld` (`self.WeaponSocketPosition`)) "AlwaysSpawn" "OverrideRootScale" self self))
  (switch `/Game/_HentaiShooter/Weapons/EWeaponsType` (`/Game/_HentaiShooter/Weapons/Weapons/BP_BaseWeapon.WeaponType` _returnvalue)
    (:`NewEnumerator0`
      (bind _asbp_pistol (cast `/Game/_HentaiShooter/Weapons/Weapons/BP_Pistol` _returnvalue)
        (:`then`
          (bind _bp_weaponcomponent (`self.BP_WeaponComponent`)
            (:`then`
              (bind _output_get (set `/Game/_HentaiShooter/Weapons/BP_WeaponComponent.Pistol` _asbp_pistol _bp_weaponcomponent))
              (`/Game/_HentaiShooter/Weapons/BP_WeaponComponent.AddWeapon` _bp_weaponcomponent _output_get)
              (`self.K2_AttachToComponent` _asbp_pistol _weaponsocketposition "None" "KeepWorld" "SnapToTarget" "SnapToTarget" true))
            (:`else`
              (`KismetSystemLibrary.PrintString` "Faild Equip, Weapon Comp Invalid"))))
        (:`CastFailed`
          (`KismetSystemLibrary.PrintString` "Faild Equip, Cast  Pistol  Fail"))))
    (:`NewEnumerator1`
      (bind _asbp_shotgun (cast `/Game/_HentaiShooter/Weapons/Weapons/BP_Shotgun` _returnvalue))
      (bind _bp_weaponcomponent_2 (`self.BP_WeaponComponent`)
        (:`then`
          (bind _output_get_2 (set `/Game/_HentaiShooter/Weapons/BP_WeaponComponent.Shotgun` _asbp_shotgun _bp_weaponcomponent_2))
          (`/Game/_HentaiShooter/Weapons/BP_WeaponComponent.AddWeapon` _bp_weaponcomponent_2 _output_get_2)
          (`self.K2_AttachToComponent` _asbp_shotgun _weaponsocketposition "None" "KeepWorld" "SnapToTarget" "SnapToTarget" true))
        (:`else`)))
    (:`NewEnumerator2`
      (bind _asbp_fist (cast `/Game/_HentaiShooter/Weapons/Weapons/BP_Fist` _returnvalue))
      (bind _bp_weaponcomponent_3 (`self.BP_WeaponComponent`)
        (:`then`
          (bind _output_get_3 (set `/Game/_HentaiShooter/Weapons/BP_WeaponComponent.Fist` _asbp_fist _bp_weaponcomponent_3))
          (`/Game/_HentaiShooter/Weapons/BP_WeaponComponent.AddWeapon` _bp_weaponcomponent_3 _output_get_3)
          (`self.K2_AttachToComponent` _asbp_fist (`self.StaticWeaponSocket`) "None" "SnapToTarget" "SnapToTarget" "SnapToTarget" true))
        (:`else`)))
    (:`NewEnumerator3`
      (bind _asbp_lazer (cast `/Game/_HentaiShooter/Weapons/Weapons/BP_Lazer` _returnvalue))
      (bind _bp_weaponcomponent_4 (`self.BP_WeaponComponent`)
        (:`then`
          (bind _output_get_4 (set `/Game/_HentaiShooter/Weapons/BP_WeaponComponent.Laser` _asbp_lazer _bp_weaponcomponent_4))
          (`/Game/_HentaiShooter/Weapons/BP_WeaponComponent.AddWeapon` _bp_weaponcomponent_4 _output_get_4)
          (`self.K2_AttachToComponent` _asbp_lazer (`self.HeadSocket`) "None" "SnapToTarget" "SnapToTarget" "SnapToTarget" true))
        (:`else`)))
    (:`NewEnumerator4`
      (bind _asbp_bike (cast `/Game/_HentaiShooter/Weapons/Weapons/BP_Bike` _returnvalue))
      (bind _bp_weaponcomponent_5 (`self.BP_WeaponComponent`)
        (:`then`
          (bind _output_get_5 (set `/Game/_HentaiShooter/Weapons/BP_WeaponComponent.Bike` _asbp_bike _bp_weaponcomponent_5))
          (`/Game/_HentaiShooter/Weapons/BP_WeaponComponent.AddWeapon` _bp_weaponcomponent_5 _output_get_5)
          (`self.K2_AttachToComponent` _asbp_bike (`self.StaticWeaponSocket`) "None" "SnapToTarget" "SnapToTarget" "SnapToTarget" true))
        (:`else`)))
    (:`NewEnumerator5`
      (bind _asbp_bomb (cast `/Game/_HentaiShooter/Weapons/Weapons/BP_Bomb` _returnvalue))
      (bind _bp_weaponcomponent_6 (`self.BP_WeaponComponent`)
        (:`then`
          (bind _output_get_6 (set `/Game/_HentaiShooter/Weapons/BP_WeaponComponent.Bomb` _asbp_bomb _bp_weaponcomponent_6))
          (`/Game/_HentaiShooter/Weapons/BP_WeaponComponent.AddWeapon` _bp_weaponcomponent_6 _output_get_6)
          (`self.K2_AttachToComponent` _asbp_bomb (`self.WeaponSocketPosition`) "None" "SnapToTarget" "SnapToTarget" "SnapToTarget" true))
        (:`else`)))
    (:`NewEnumerator6`
      (bind _asbp_time_freezer (cast `/Game/_HentaiShooter/Weapons/Weapons/BP_TimeFreezer` _returnvalue))
      (bind _bp_weaponcomponent_7 (`self.BP_WeaponComponent`)
        (:`then`
          (bind _output_get_7 (set `/Game/_HentaiShooter/Weapons/BP_WeaponComponent.TimeFreezer` _asbp_time_freezer _bp_weaponcomponent_7))
          (`/Game/_HentaiShooter/Weapons/BP_WeaponComponent.AddWeapon` _bp_weaponcomponent_7 _output_get_7)
          (`self.K2_AttachToComponent` _asbp_time_freezer (`self.StaticWeaponSocket`) "None" "SnapToTarget" "SnapToTarget" "SnapToTarget" true))
        (:`else`)))
    (:`NewEnumerator7`
      (bind _asbp_shining (cast `/Game/_HentaiShooter/Weapons/Weapons/BP_Shining` _returnvalue))
      (bind _bp_weaponcomponent_8 (`self.BP_WeaponComponent`)
        (:`then`
          (bind _output_get_8 (set `/Game/_HentaiShooter/Weapons/BP_WeaponComponent.Shining` _asbp_shining _bp_weaponcomponent_8))
          (`/Game/_HentaiShooter/Weapons/BP_WeaponComponent.AddWeapon` _bp_weaponcomponent_8 _output_get_8)
          (`self.K2_AttachToComponent` _asbp_shining (`self.StaticWeaponSocket`) "None" "SnapToTarget" "SnapToTarget" "SnapToTarget" true))
        (:`else`)))
    (:`NewEnumerator8`
      (bind _asbp_sparkle (cast `/Game/_HentaiShooter/Weapons/Weapons/BP_Sparkle` _returnvalue))
      (bind _bp_weaponcomponent_9 (`self.BP_WeaponComponent`)
        (:`then`
          (set `/Game/_HentaiShooter/Weapons/BP_WeaponComponent.Sparkle` _asbp_sparkle _bp_weaponcomponent_9)
          (`/Game/_HentaiShooter/Weapons/BP_WeaponComponent.AddWeapon` _bp_weaponcomponent_9 _asbp_sparkle)
          (`self.K2_AttachToComponent` _asbp_sparkle (`self.StaticWeaponSocket`) "None" "SnapToTarget" "SnapToTarget" "SnapToTarget" true))
        (:`else`)))
    (:`NewEnumerator10`
      (bind _asbp_hp (cast `/Game/_HentaiShooter/Weapons/Weapons/BP_HP` _returnvalue))
      (bind _bp_weaponcomponent_10 (`self.BP_WeaponComponent`)
        (:`then`
          (bind _output_get_9 (set `/Game/_HentaiShooter/Weapons/BP_WeaponComponent.HP` _asbp_hp _bp_weaponcomponent_10))
          (set `/Game/_HentaiShooter/Weapons/Weapons/BP_HP.HealthComponent` (`self.BP_HealthComponent`) _output_get_9)
          (`/Game/_HentaiShooter/Weapons/BP_WeaponComponent.AddWeapon` _bp_weaponcomponent_10 _asbp_hp)
          (`self.K2_AttachToComponent` _asbp_hp (`self.StaticWeaponSocket`) "None" "SnapToTarget" "SnapToTarget" "SnapToTarget" true))
        (:`else`)))))

(fn `SetDashForwardAxis`
  (set `self.DashForwardAxis` (`self.GetInputAxisValue`))
  (return))

(fn `SetDashRightAxis`
  (set `self.DashRightAxis` (`self.GetInputAxisValue`))
  (return))

(fn `UserConstructionScript`)