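; BP_RangedWeapon is a weapon actor that fires projectiles through its Shoot event.
; Shoot spawns a Projectile at the weapon's own location and rotation regardless of collision, with the weapon as owner, passing on its TeamNumber and a fixed damage value.
; It then plays a sound at that location.
; The default events are disabled stubs, and nothing here limits fire rate or ammo.
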(event `/Game/_HentaiShooter/Weapons/BPI_Weapon.Shoot`
  (bind (_returnvalue_location _returnvalue_rotation) (`KismetMathLibrary.BreakTransform` (`self.GetTransform`)))
  (`|SpawnActorFromClass` (`self.Projectile`) (`KismetMathLibrary.MakeTransform` _returnvalue_location _returnvalue_rotation) "AlwaysSpawn" "OverrideRootScale" self (`self.TeamNumber`) 20.0 null)
  (`GameplayStatics.PlaySoundAtLocation` null _returnvalue_location (struct) 1.0 1.0 0.0 null null null null))

(fn `UserConstructionScript`
  (`parent.UserConstructionScript`))