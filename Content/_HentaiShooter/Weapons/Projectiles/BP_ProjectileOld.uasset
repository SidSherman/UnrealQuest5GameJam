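; Projectile actor that flies straight along its forward vector with a swept move each tick, sizing its capsule and setting its lifespan on begin play.
; Overlaps apply damage credited to the Instigator, or to player 0's controller if none is valid, then optionally destroy the projectile.
; The Instigator itself is spared, triggering only a debug print.
; Overlaps increment a hit count, but the penetration-limit check is disconnected.
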(event `self.ReceiveTick`
  (params (DeltaSeconds :type "Float (single-precision)"))
  (`self.K2_AddActorWorldOffset` (* (`self.GetActorForwardVector`) (* DeltaSeconds (`self.Speed`))) true))

(event `self.ReceiveBeginPlay`
  (`self.SetLifeSpan` (`self.Lifetime`))
  (`CapsuleComponent.SetCapsuleSize` (`self.Capsule`) (* (`self.DefaultRadius`) (`self.Size`)) (* (`self.DefaultHalfHeight`) (`self.Size`)) true))

(event `Damage Actor`
  (params (Actor :type "Actor Object Reference"))
  (bind _instigator (`self.Instigator`))
  (`/Engine/EditorBlueprintResources/StandardMacros.IsValid` _instigator
    (:`Is Valid`
      (if (!= Actor _instigator)
        (`GameplayStatics.ApplyDamage` Actor (`self.Damage`) (`Pawn.GetController` _instigator) self "/Script/Engine.DamageType")
        (if (`self.bShouldDestroyAfterDamage`) :!label _label
          (`self.K2_DestroyActor`))
        (else
          (`KismetSystemLibrary.PrintString` "Hello"))))
    (:`Is Not Valid`
      (`GameplayStatics.ApplyDamage` Actor (`self.Damage`) (`GameplayStatics.GetPlayerController` 0) self "/Script/Engine.DamageType")
      (goto _label))))

(event `self.ReceiveActorBeginOverlap`
  (params (OtherActor :type "Actor Object Reference"))
  (`self.Damage Actor` OtherActor)
  (`/Engine/EditorBlueprintResources/StandardMacros.IncrementInt` (`self.HitCount`)))

(fn `UserConstructionScript`)