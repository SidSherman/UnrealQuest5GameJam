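; BP_RangedEnemyZDCharacter is a ranged enemy character that fires a child-actor weapon when it attacks.
; On Attack it sets the world rotation of its weapon socket component to a look-at rotation, then sends a shoot message to the weapon's child actor.
; BeginPlay and construction defer to the parent class, and Tick is disabled.
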(event `self.ReceiveBeginPlay`
  (`parent.ReceiveBeginPlay`))

(event `/Game/UnrealQuest5/Blueprints/Characters/BPI_Character.Attack`
  (`SceneComponent.K2_SetWorldRotation` (`self.RotationWeaponSocket`) (`self.LookAtRotation`) false false)
  (message `/Game/UnrealQuest5/Blueprints/Weapons/BPI_Weapon.Shoot` (`ChildActorComponent.ChildActor` (`self.Weapon`))))

(fn `UserConstructionScript`
  (`parent.UserConstructionScript`))