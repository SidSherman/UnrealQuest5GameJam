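; BP_OverlappingProjectile is a projectile Blueprint that deals repeated area damage to actors inside its capsule.
; On BeginPlay it runs the parent logic, then starts a looping one-second timer.
; Each timer tick prints a leftover-style "Hello" debug string and calls DamageActor on every actor currently overlapping the Capsule.
; Damage relies on this periodic polling, as the overlap and Tick events are disabled.
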(event `self.ReceiveBeginPlay`
  (`parent.ReceiveBeginPlay`)
  (`KismetSystemLibrary.K2_SetTimerDelegate` (delegate `DamageAllActorsByTimer`) 1.0 true -1.0))

(event `DamageAllActorsByTimer`
  (`KismetSystemLibrary.PrintString` "Hello")
  (for _array_element (`PrimitiveComponent.GetOverlappingActors` (`self.Capsule`) null)
    (`self.Damage Actor` _array_element)))

(fn `UserConstructionScript`
  (`parent.UserConstructionScript`))