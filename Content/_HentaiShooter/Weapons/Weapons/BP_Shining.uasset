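; BP_Shining is a weapon that fires repeated timed bursts, damaging actors that enter its hitbox.
; StartShoot runs a looping Shoot timer, with a negative initial delay cancelling the first wait.
; Each shot enables and reveals the hitbox, restarts the Explosion flipbook, then schedules StopShoot to hide and disable both after ActiveTime.
; Overlaps during that window apply damage credited to the Instigator's controller, excluding the Instigator itself.
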(event `/Game/_HentaiShooter/Weapons/BPI_Weapon.StartShoot`
  (bind _shootingrate (`self.ShootingRate`))
  (bind _returnvalue (`KismetSystemLibrary.K2_SetTimerDelegate` (delegate `/Game/_HentaiShooter/Weapons/BPI_Weapon.Shoot`) _shootingrate true (* _shootingrate -1.0)))
  (set `self.ShootingTimer` _returnvalue))

(event `/Game/_HentaiShooter/Weapons/BPI_Weapon.Shoot`
  (bind _explosion (`self.Explosion`))
  (`PrimitiveComponent.SetCollisionEnabled` (`self.HitBox`) "QueryOnly")
  (`SceneComponent.SetHiddenInGame` _explosion false false)
  (`SceneComponent.SetHiddenInGame` (`self.HitBox`) false false)
  (`PaperFlipbookComponent.SetPlaybackPositionInFrames` _explosion 0 false)
  (`PaperFlipbookComponent.PlayFromStart` _explosion)
  (bind _returnvalue (`KismetSystemLibrary.K2_SetTimerDelegate` (delegate `/Game/_HentaiShooter/Weapons/BPI_Weapon.StopShoot`) (`self.ActiveTime`)))
  (set `self.ActivateTimerHandle` _returnvalue))

(event `/Game/_HentaiShooter/Weapons/BPI_Weapon.StopShoot`
  (bind _explosion (`self.Explosion`))
  (`PrimitiveComponent.SetCollisionEnabled` (`self.HitBox`) "NoCollision")
  (`SceneComponent.SetHiddenInGame` _explosion true false)
  (`SceneComponent.SetHiddenInGame` (`self.HitBox`) true false)
  (`PaperFlipbookComponent.Stop` _explosion))

(event `self.HitBox.OnComponentBeginOverlap`
  (params (OverlappedComponent :type "PrimitiveComponent Object Reference") (OtherActor :type "Actor Object Reference") (OtherComp :type "PrimitiveComponent Object Reference") (OtherBodyIndex :type Integer) (bFromSweep :type Boolean) (SweepResult :type "HitResult Structure (by ref)"))
  (bind _instigator (`self.Instigator`))
  (`/Engine/EditorBlueprintResources/StandardMacros.IsValid` _instigator
    (:`Is Valid`
      (if (!= OtherActor _instigator)
        (`GameplayStatics.ApplyDamage` OtherActor (`self.Damage`) (`Pawn.GetController` _instigator) self "/Script/Engine.DamageType")))))

(fn `UserConstructionScript`
  (`parent.UserConstructionScript`))