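; BP_TimeFreezer is a weapon Blueprint that periodically freezes enemies in time.
; StartShoot sets a timer for Shoot, which zeroes enemy time dilation through the owner's BP_SpawnManager component.
; After ActiveTime, StopShoot restores normal enemy speed and restarts the cycle if that component is valid.
; A separate Set CustomTimeDilation graph offsets global dilation on the owner and its child actors.
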(event `self.StartShoot`
  (bind _returnvalue (`KismetSystemLibrary.K2_SetTimerDelegate` (delegate `self.Shoot`) (`self.ShootingRate`)))
  (set `self.ShootingTimeHandle` _returnvalue))

(event `self.Shoot`
  (bind _returnvalue (`self.GetComponentByClass` (`self.GetOwner`) "/Game/UnrealQuest5/Blueprints/Components/Spawner/BP_SpawnManager.BP_SpawnManager_C"))
  (`/Engine/EditorBlueprintResources/StandardMacros.IsValid` _returnvalue
    (:`Is Valid`
      (`/Game/UnrealQuest5/Blueprints/Components/Spawner/BP_SpawnManager.SetEnemiesTimeDilation` _returnvalue 0.0))
    (:`Is Not Valid`
      _))
  (bind _returnvalue_2 (`KismetSystemLibrary.K2_SetTimerDelegate` (delegate `self.StopShoot`) (`self.ActiveTime`)))
  (set `self.ActivateTimeHandle` _returnvalue_2))

(event `self.StopShoot`
  (bind _returnvalue (`self.GetComponentByClass` (`self.GetOwner`) "/Game/UnrealQuest5/Blueprints/Components/Spawner/BP_SpawnManager.BP_SpawnManager_C"))
  (`/Engine/EditorBlueprintResources/StandardMacros.IsValid` _returnvalue
    (:`Is Valid`
      (`/Game/UnrealQuest5/Blueprints/Components/Spawner/BP_SpawnManager.SetEnemiesTimeDilation` _returnvalue 1.0)
      (`self.StartShoot`))))

(fn `UserConstructionScript`
  (`parent.UserConstructionScript`))