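; Bomb projectile that explodes when it overlaps an actor from another team, any actor if friendly fire is on, or just before its lifetime ends.
; Explosion switches the Sphere to query-only collision, plays a sound and damages every actor overlapping the Sphere, with no team filter.
; It then spawns the explosion FX and calls OnHitEvent.
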(event `self.ReceiveBeginPlay`
  (`parent.ReceiveBeginPlay`)
  (`KismetSystemLibrary.Delay` (- (`self.Lifetime`) 0.1))
  (`self.Explode`))

(event `self.ReceiveActorBeginOverlap`
  (params (OtherActor :type "Actor Object Reference"))
  ;[1 1 1] Explode bomb
  (if (`self.bIsExploding`)
    _
    (elif (`self.bIsFriendleFireActive`)
      (`self.Explode` :!label _label)
      (else
        (bind _teamnumber (message `/Game/UnrealQuest5/Blueprints/Items/BPI_Item.GetTeamNumber` OtherActor))
        (if (!= _teamnumber (`self.TeamNumber`))
          (goto _label))))))

(event `Explode`
  (bind _returnvalue_location (`KismetMathLibrary.BreakTransform` (`self.GetTransform`)))
  (bind _returnvalue (`self.GetTransform`))
  ;[1 1 1] Explode bomb
  (set `self.bIsExploding` true)
  (bind _sphere (`self.Sphere`)
    (:`then`
      (`PrimitiveComponent.SetCollisionEnabled` _sphere "QueryOnly")
      (`GameplayStatics.PlaySoundAtLocation` "/Game/Dev/Temp/Sounds/A_grenadeExplosion_Cue.A_grenadeExplosion_Cue" _returnvalue_location (struct) 1.0 1.0 0.0 null null null null)
      (bind _sphere_2 (`self.Sphere`)
        (:`then`
          (for _array_element (`PrimitiveComponent.GetOverlappingActors` _sphere_2 "/Script/Engine.Actor")
            (`self.ApplyDamageToActor` _array_element))
          (`|SpawnActorFromClass` (`self.ExplosionFX`) (`KismetMathLibrary.MakeTransform` (`KismetMathLibrary.MakeVector` (.x (.location _returnvalue)) (.y (.location _returnvalue)) (+ (.z (.location _returnvalue)) 5.0)) (struct :`Roll` -90.0) (2.5 2.5 2.5)) "AlwaysSpawn" "OverrideRootScale" null null)
          (`self.OnHit_Event`))
        (:`else`)))
    (:`else`)))

(fn `UserConstructionScript`
  (`parent.UserConstructionScript`))