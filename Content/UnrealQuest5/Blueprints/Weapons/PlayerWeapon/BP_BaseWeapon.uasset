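; BP_BaseWeapon is a base player weapon that holds team and combat stats for the game's weapon types.
; On BeginPlay it loads the first-tier values from DT_DefaultWeaponStats using a row picked by WeaponType, then caches the game state.
; It then takes the team number from a valid instigator.
; UpdateTimers restarts shooting on auto-attack weapons through StopShoot and StartShoot.
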(event `self.ReceiveBeginPlay`
  (bind _returnvalue (`self.GetInstigator`))
  ;[1 1 1] BeginPlay
  (`|ExecutionSequence`
    (:`then_0`
      (`self.SetStats`)
      (bind _asbp_game_state (cast `/Game/UnrealQuest5/Blueprints/General/BP_GameState` (`GameplayStatics.GetGameState`)))
      (set `self.GameState` _asbp_game_state))
    (:`then_1`
      (`/Engine/EditorBlueprintResources/StandardMacros.IsValid` _returnvalue
        (:`Is Valid`
          (bind _teamnumber (message `/Game/UnrealQuest5/Blueprints/Items/BPI_Item.GetTeamNumber` _returnvalue))
          (message `/Game/UnrealQuest5/Blueprints/Items/BPI_Item.SetTeamNumber` self _teamnumber))))))

(event `/Game/UnrealQuest5/Blueprints/Items/BPI_Item.SetTeamNumber`
  (params (TeamNumber :type Byte))
  ;[1 1 1] Set Team Number
  (set `self.TeamNumber` TeamNumber))

(event `SetStats`
  ;[1 1 1] Set Weapon Stats from Data Table
  (bind _returnvalue (`|GetDataTableRow` "/Game/UnrealQuest5/Blueprints/Weapons/DT_DefaultWeaponStats.DT_DefaultWeaponStats" (select `/Game/UnrealQuest5/Blueprints/Weapons/EWeaponsType` (`self.WeaponType`) :`NewEnumerator0` "Pistol" :`NewEnumerator1` "Shotgun" :`NewEnumerator2` "Fist" :`NewEnumerator3` "Laser" :`NewEnumerator4` "Bike" :`NewEnumerator5` "Bomb" :`NewEnumerator6` "TimeFreezer" :`NewEnumerator7` "Shining" :`NewEnumerator8` "Sparkle" :`NewEnumerator10` "HP" :`NewEnumerator11` "Sword" :`NewEnumerator12` "Stamina" :`NewEnumerator13` "RotatingSword" :`NewEnumerator14` "Shield" :!type "Name"))
    (:`then`
      (`|ExecutionSequence`
        (:`then_0`
          (set `self.Damage` (`|GetArrayItem` (break `/Game/UnrealQuest5/Blueprints/Weapons/WeaponStats` _returnvalue))))
        (:`then_1`
          (set `self.Size` (`|GetArrayItem` (`.Size_17_37DCE96A4C44339D0FF10CAF8F1975E3` (break `/Game/UnrealQuest5/Blueprints/Weapons/WeaponStats` _returnvalue)))))
        (:`then_2`
          (set `self.ShootingRate` (`|GetArrayItem` (`.Rate_18_700A31494A1C42C3C0CF8A9475E5ECC9` (break `/Game/UnrealQuest5/Blueprints/Weapons/WeaponStats` _returnvalue)))))
        (:`then_3`
          (set `self.ProjectileCount` (`|GetArrayItem` (`.ProjectileCount_19_B75409154477CD454D667BA0672A1428` (break `/Game/UnrealQuest5/Blueprints/Weapons/WeaponStats` _returnvalue)))))
        (:`then_4`
          (set `self.ActiveTime` (`|GetArrayItem` (`.ActiveTime_20_81FE32664A4654363DA7F5B32C9CD936` (break `/Game/UnrealQuest5/Blueprints/Weapons/WeaponStats` _returnvalue)))))
        (:`then_5`
          (set `self.Spreading` (`|GetArrayItem` (`.Spreading_59_3300FBFD475D0721FDB17CA170585120` (break `/Game/UnrealQuest5/Blueprints/Weapons/WeaponStats` _returnvalue)))))))))

(event `UpdateTimers`
  ;[1 1 1] Update Timers
  (if (`self.bIsAutoAttack`)
    (`/Game/UnrealQuest5/Blueprints/Weapons/BPI_Weapon.StopShoot`)
    (`/Game/UnrealQuest5/Blueprints/Weapons/BPI_Weapon.StartShoot`)))

(fn `GetTeamNumber`
  (returns (TeamNumber :type Byte))
  (return (`self.TeamNumber`)))

(fn `UserConstructionScript`)