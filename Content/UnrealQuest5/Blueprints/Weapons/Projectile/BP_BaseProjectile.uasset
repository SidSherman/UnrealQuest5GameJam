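; Base projectile actor that flies straight ahead and damages actors on a different team.
; On BeginPlay it takes the team number from its instigator, binds its hit handler and sets its lifespan.
; Tick moves it along its forward vector with a swept offset rather than a movement component.
; Overlapping an actor with a different team number applies damage and fires the OnHit dispatcher, whose bound handler destroys the projectile.
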(event `self.ReceiveBeginPlay`
  (bind _returnvalue (`self.GetInstigator`))
  (`/Engine/EditorBlueprintResources/StandardMacros.IsValid` _returnvalue
    (:`Is Valid`
      (bind _teamnumber (message `/Game/UnrealQuest5/Blueprints/Weapons/BPI_Item.GetTeamNumber` _returnvalue))
      (`/Game/UnrealQuest5/Blueprints/Weapons/BPI_Item.SetTeamNumber` _teamnumber))
    (:`Is Not Valid`
      _))
  (add `self.OnHit` (delegate `OnHit_Event`))
  (`self.SetLifeSpan` (`self.Lifetime`)))

(event `OnHit_Event`
  (`self.K2_DestroyActor`))

(event `self.ReceiveActorBeginOverlap`
  (params (OtherActor :type "Actor Object Reference"))
  (bind _teamnumber (message `/Game/UnrealQuest5/Blueprints/Weapons/BPI_Item.GetTeamNumber` OtherActor))
  (if (!= _teamnumber (`self.TeamNumber`))
    (`self.ApplyDamageToActor` OtherActor)
    (`self.OnHit`)))

(event `self.ReceiveTick`
  (params (DeltaSeconds :type "Float (single-precision)"))
  (`self.K2_AddActorWorldOffset` (* (`self.GetActorForwardVector`) (* DeltaSeconds (`self.Speed`))) true))

(event `/Game/UnrealQuest5/Blueprints/Weapons/BPI_Item.SetTeamNumber`
  (params (TeamNumber :type Byte))
  (set `self.TeamNumber` TeamNumber))

(fn `ApplyDamageToActor`
  (params (InputPin :type "Actor Object Reference"))
  (bind _teamnumber (message `/Game/UnrealQuest5/Blueprints/Weapons/BPI_Item.GetTeamNumber` InputPin))
  (if (!= _teamnumber (`self.TeamNumber`))
    (`GameplayStatics.ApplyDamage` InputPin (`self.Damage`) null self)))

(fn `GetTeamNumber`
  (returns (TeamNumber :type Byte))
  (return (`self.TeamNumber`)))

(fn `UserConstructionScript`)