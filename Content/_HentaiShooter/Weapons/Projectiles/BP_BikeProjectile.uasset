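; BP_BikeProjectile is a weapon projectile that damages actors it overlaps and ricochets off surfaces.
; Each tick, after the parent tick, it runs a short forward Visibility trace and, on a hit, reflects its heading off the surface normal, changing only yaw.
; Each bounce increments HitCount, and the projectile destroys itself once that count reaches PenetratingPower.
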(event `self.ReceiveActorBeginOverlap`
  (params (OtherActor :type "Actor Object Reference"))
  (`self.Damage Actor` OtherActor))

(event `self.ReceiveTick`
  (params (DeltaSeconds :type "Float (single-precision)"))
  (bind _returnvalue (`self.K2_GetActorLocation`))
  (bind (_returnvalue_roll _returnvalue_pitch) (`KismetMathLibrary.BreakRotator` (`self.K2_GetActorRotation`)))
  (bind _hitcount (`self.HitCount`))
  (`parent.ReceiveTick` DeltaSeconds)
  (bind (_outhit _returnvalue_2) (`KismetSystemLibrary.LineTraceSingle` _returnvalue (+ _returnvalue (* (`self.GetActorForwardVector`) 50.0)) "TraceTypeQuery1" true))
  (if _returnvalue_2
    (bind (_vector _rotation) (`/Game/_HentaiShooter/Core/BP_FunctionLibrary.GetRefrectionVectorAndRotator` (`self.GetActorForwardVector`) (`.Normal` (`GameplayStatics.BreakHitResult` _outhit))))
    (`self.K2_SetActorRotation` (`KismetMathLibrary.MakeRotator` _returnvalue_roll _returnvalue_pitch (.yaw _rotation)) true)
    (`/Engine/EditorBlueprintResources/StandardMacros.IncrementInt` _hitcount
      (:`  `
        (if (>= _hitcount (`self.PenetratingPower`))
          (`self.K2_DestroyActor`))))))

(fn `UserConstructionScript`
  (`parent.UserConstructionScript`))