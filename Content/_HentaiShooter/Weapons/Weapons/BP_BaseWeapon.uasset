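; Base weapon Blueprint that loads its stats from DT_DefaultWeaponStats by WeaponType on BeginPlay and caches the game state.
; StartShoot runs a looping timer at ShootingRate, offset to fire immediately, and StopShoot clears a flag so the next tick cancels it.
; Each shot spawns ProjectileCount projectiles at the barrel with random yaw spread, passing ProjectileCount as penetrating power instead of the loaded PenetrationPower.
; Special skill and reload events are empty stubs.
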(event `SetStats`
  (bind _returnvalue (`|GetDataTableRow` "/Game/_HentaiShooter/Weapons/DT_DefaultWeaponStats.DT_DefaultWeaponStats" (select `/Game/_HentaiShooter/Weapons/EWeaponsType` (`self.WeaponType`) :`NewEnumerator0` "Pistol" :`NewEnumerator1` "Shotgun" :`NewEnumerator2` "Fist" :`NewEnumerator3` "Laser" :`NewEnumerator4` "Bike" :`NewEnumerator5` "Bomb" :`NewEnumerator6` "TimeFreeze" :`NewEnumerator7` "Shining" :`NewEnumerator8` "Sparkle" :`NewEnumerator10` "HP" :!type "Name"))
    (:`then`
      (`|ExecutionSequence`
        (:`then_0`
          (set `self.Damage` (`|GetArrayItem` (break `/Game/_HentaiShooter/Weapons/WeaponStats` _returnvalue))))
        (:`then_1`
          (set `self.Size` (`|GetArrayItem` (`.Size_17_37DCE96A4C44339D0FF10CAF8F1975E3` (break `/Game/_HentaiShooter/Weapons/WeaponStats` _returnvalue)))))
        (:`then_2`
          (set `self.ShootingRate` (`|GetArrayItem` (`.Rate_18_700A31494A1C42C3C0CF8A9475E5ECC9` (break `/Game/_HentaiShooter/Weapons/WeaponStats` _returnvalue)))))
        (:`then_3`
          (set `self.ProjectileCount` (`|GetArrayItem` (`.ProjectileCount_19_B75409154477CD454D667BA0672A1428` (break `/Game/_HentaiShooter/Weapons/WeaponStats` _returnvalue)))))
        (:`then_4`
          (set `self.ActiveTime` (`|GetArrayItem` (`.ActiveTime_20_81FE32664A4654363DA7F5B32C9CD936` (break `/Game/_HentaiShooter/Weapons/WeaponStats` _returnvalue)))))
        (:`then_5`
          (set `self.PenetrationPower` (`|GetArrayItem` (`.PenetrationPower_56_CECD67664815FCA7ED1D3395FC00BD61` (break `/Game/_HentaiShooter/Weapons/WeaponStats` _returnvalue)))))
        (:`then_6`
          (set `self.Spreading` (`|GetArrayItem` (`.Spreading_59_3300FBFD475D0721FDB17CA170585120` (break `/Game/_HentaiShooter/Weapons/WeaponStats` _returnvalue)))))))))

(event `self.ReceiveBeginPlay`
  ;[1 1 1] BeginPlay
  (`self.SetStats`)
  (bind _asbp_game_state (cast `/Game/UnrealQuest5/Blueprints/General/BP_GameState` (`GameplayStatics.GetGameState`)))
  (set `self.GameState` _asbp_game_state))

(event `UpdateTimers`
  (`/Game/_HentaiShooter/Weapons/BPI_Weapon.StopShoot`)
  (`/Game/_HentaiShooter/Weapons/BPI_Weapon.StartShoot`))

(event `/Game/_HentaiShooter/Weapons/BPI_Weapon.StartShoot`
  (bind _shootingrate (`self.ShootingRate`))
  ;[1 1 1] ShootingLogic
  (set `self.bIsShooting` true)
  (`KismetSystemLibrary.K2_ClearAndInvalidateTimerHandle` (`self.ShootingTimer`))
  (bind _returnvalue (`KismetSystemLibrary.K2_SetTimerDelegate` (delegate `/Game/_HentaiShooter/Weapons/BPI_Weapon.Shoot`) _shootingrate true (* _shootingrate -1.0)))
  (set `self.ShootingTimer` _returnvalue))

(event `/Game/_HentaiShooter/Weapons/BPI_Weapon.Shoot`
  (bind _size (`self.Size`))
  (bind _returnvalue (`SceneComponent.K2_GetComponentToWorld` (`self.BarrelLocation`)))
  ;[1 1 1] ShootingLogic
  (if (`self.bIsShooting`)
    (for _ (range (`self.ProjectileCount`))
      (`|SpawnActorFromClass` (`self.CurrentProjectile`) (`KismetMathLibrary.MakeTransform` (.location _returnvalue) (`KismetMathLibrary.MakeRotator` -90.0 (.pitch (.rotation _returnvalue)) (+ (.yaw (.rotation _returnvalue)) (`KismetMathLibrary.RandomFloatInRange` (* (`self.Spreading`) -1.0) (`self.Spreading`)))) (`KismetMathLibrary.MakeVector` _size _size _size)) "AdjustIfPossibleButAlwaysSpawn" "OverrideRootScale" self (`self.ActiveTime`) (`self.Damage`) (`self.Size`) (`self.ProjectileCount`) (`self.Instigator`))
      (`GameplayStatics.PlaySound2D` null 0.6 1.0 0.0 null null))
    (else
      (`KismetSystemLibrary.K2_ClearAndInvalidateTimerHandle` (`self.ShootingTimer`)))))

(event `/Game/_HentaiShooter/Weapons/BPI_Weapon.SpetialSkill`
  ;[1 1 1] ShootingLogic
)

(event `/Game/_HentaiShooter/Weapons/BPI_Weapon.StopShoot`
  ;[1 1 1] ShootingLogic
  (set `self.bIsShooting` false))

(event `StartReload`
  ;[1 1 1] ShootingLogic
)

(event `StopReload`
  ;[1 1 1] ShootingLogic
)

(fn `UserConstructionScript`)