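; Turret character with a sprite that deals contact damage and handles its own death.
; On death it unpossesses, disables health and collision, greys the sprite, fades opacity on a timeline, then spawns loot and destroys itself.
; Capsule hits on actors of a different team number apply damage and launch characters horizontally along the impact normal, gated by a one-second recharge timer.
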(event `self.OnDeath_Event`
  ;[1 1 1] Death
  (set `self.bIsDead` true)
  (`Controller.UnPossess` (`self.GetController`))
  (`ActorComponent.Deactivate` (`self.BPC_HealthComponent`))
  (`PrimitiveComponent.SetCollisionEnabled` (`self.CapsuleComponent`) "NoCollision")
  (`PaperFlipbookComponent.SetSpriteColor` (`self.Sprite`) (struct :`R` 0.5 :`G` 0.5 :`B` 0.5 :`A` 1.0))
  (bind (_direction _alpha) (`Timeline|DeathTimeLine` :!via `PlayFromStart`)
    (:`Update`
      (`MaterialInstanceDynamic.SetScalarParameterValue` (`self.SpriteMaterial`) "Opacity" (`KismetMathLibrary.Lerp` 2.0 0.0 _alpha)))
    (:`Finished`
      ;;[1 1 1] SpawnLoot
      (`self.SpawnLoot`)
      (`self.K2_DestroyActor`))))

(event `self.CapsuleComponent.OnComponentHit`
  (params (HitComponent :type "PrimitiveComponent Object Reference") (OtherActor :type "Actor Object Reference") (OtherComp :type "PrimitiveComponent Object Reference") (NormalImpulse :type "Vector Structure") (Hit :type "HitResult Structure (by ref)"))
  ;[1 1 1] DamageOnhit
  (if (`self.bCanAttackOnOverlap`)
    (`KismetSystemLibrary.PrintString` (`KismetSystemLibrary.GetDisplayName` OtherActor))
    (bind _teamnumber (message `/Game/UnrealQuest5/Blueprints/Weapons/BPI_Item.GetTeamNumber` OtherActor))
    (if (!= _teamnumber (`self.TeamNumber`))
      (`KismetSystemLibrary.K2_SetTimerDelegate` (delegate `RechargeOnOverlapAttack`) 1.0)
      (set `self.bCanAttackOnOverlap` false)
      (`GameplayStatics.ApplyDamage` OtherActor (`self.BaseHitDamage`))
      (bind _ascharacter (cast `Character` OtherActor))
      (`self.LaunchCharacter` _ascharacter (* (`KismetMathLibrary.MakeVector` (.x Hit_ImpactNormal) (.y Hit_ImpactNormal)) -500.0) false false))))

(event `RechargeOnOverlapAttack`
  ;[1 1 1] DamageOnhit
  (set `self.bCanAttackOnOverlap` true))

(fn `UserConstructionScript`
  (`parent.UserConstructionScript`))