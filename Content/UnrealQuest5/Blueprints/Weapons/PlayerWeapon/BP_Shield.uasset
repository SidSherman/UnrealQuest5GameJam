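; BP_Shield is a player weapon that acts as a regenerating charge-based shield, reusing the weapon's projectile count as its charge capacity.
; Any damage removes one charge and starts the non-looping shoot timer; each Shoot restores one charge and re-arms it until full.
; A text render shows the current charge count, and it and the paper sprite hide at zero, then reappear when a charge returns.
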(event `self.ReceiveBeginPlay`
  (`parent.ReceiveBeginPlay`)
  (set `self.CurrentProjectileCount` (`self.ProjectileCount`)))

(event `/Game/UnrealQuest5/Blueprints/Weapons/BPI_Weapon.StopShoot`
  (`KismetSystemLibrary.K2_ClearAndInvalidateTimerHandle` (`self.ShootingTimeHandle`)))

(event `/Game/UnrealQuest5/Blueprints/Weapons/BPI_Weapon.StartShoot`
  (bind _returnvalue (`KismetSystemLibrary.K2_SetTimerDelegate` (delegate `/Game/UnrealQuest5/Blueprints/Weapons/BPI_Weapon.Shoot`) (`self.ShootingRate`)))
  (set `self.ShootingTimeHandle` _returnvalue))

(event `/Game/UnrealQuest5/Blueprints/Weapons/BPI_Weapon.Shoot`
  (bind _output_get (set `self.CurrentProjectileCount` (`KismetMathLibrary.Clamp` (+ (`self.CurrentProjectileCount`) 1) 0 (`self.ProjectileCount`))))
  (`TextRenderComponent.K2_SetText` (`self.TextRender`) (`KismetTextLibrary.Conv_IntToText` _output_get))
  (`SceneComponent.SetHiddenInGame` (`self.PaperSprite`) false false)
  (`SceneComponent.SetHiddenInGame` (`self.TextRender`) false false)
  (if (>= (`self.CurrentProjectileCount`) (`self.ProjectileCount`))
    (`/Game/UnrealQuest5/Blueprints/Weapons/BPI_Weapon.StopShoot`)
    (else
      (`/Game/UnrealQuest5/Blueprints/Weapons/BPI_Weapon.StartShoot`))))

(event `self.ReceiveAnyDamage`
  (params (Damage :type "Float (single-precision)") (DamageType :type "DamageType Object Reference") (InstigatedBy :type "Controller Object Reference") (DamageCauser :type "Actor Object Reference"))
  (bind _output_get (set `self.CurrentProjectileCount` (`KismetMathLibrary.Clamp` (- (`self.CurrentProjectileCount`) 1) 0 (`self.ProjectileCount`))))
  (`TextRenderComponent.K2_SetText` (`self.TextRender`) (`KismetTextLibrary.Conv_IntToText` _output_get))
  (if (> _output_get 0)
    (`/Game/UnrealQuest5/Blueprints/Weapons/BPI_Weapon.StartShoot`)
    (else
      (`SceneComponent.SetHiddenInGame` (`self.PaperSprite`) true false)
      (`SceneComponent.SetHiddenInGame` (`self.TextRender`) true false)
      (`/Game/UnrealQuest5/Blueprints/Weapons/BPI_Weapon.StartShoot`))))

(fn `UserConstructionScript`
  (`parent.UserConstructionScript`))